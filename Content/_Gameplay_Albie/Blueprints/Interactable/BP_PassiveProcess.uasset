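; Interactable laundry station that processes placed items passively on a timer, extending its parent's processing logic.
; Hold interact starts processing if it is idle and CanBeProcessed passes, which checks only the first placed object for a valid BP_LaundryItem.
; A looping timer drives the parent's progress update until FinishProcess clears it.
; Tap interact toggles delicate mode while CurrentTime is within DelicateSwitchTime, with debug prints for mode and progress.
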(event Custom|ProcessItems
  ;[0.05 0.05 0.05] Process Items
  (Variables|Default|SetIsActive true)
  (|CallParentFunction)
  (Utilities|Time|SetTimerbyEvent (delegate Custom|UpdateProgress) 0.1 true))

(event Custom|UpdateProgress
  ;[0.05 0.05 0.05] Update Progress
  (|CallParentFunction)
  ;[1 1 1] Debug
  (Development|PrintString (Utilities|String|ToString(Float) (Variables|Default|GetCurrentTime)) true false "(R=0.000000,G=1.000000,B=0.008285,A=1.000000)" 0.1))

(event EventFinishProcess
  ;[0.05 0.05 0.05] Finish Process
  (Variables|Default|SetIsActive false)
  (Utilities|Time|ClearTimerbyFunctionName 0 "UpdateProgress")
  (|CallParentFunction))

(event EventHoldInteract
  (params (Player :type BP%20Character%20Object%20Reference))
  ;[0.05 0.05 0.05] Begin process if not active already
  (if (CallFunction|CanbeProcessed)
    (if (not (Variables|Default|GetIsActive))
      (CallFunction|ProcessItems))))

(event EventTapInteract
  (params (Player :type BP%20Character%20Object%20Reference))
  ;[0.05 0.05 0.05] Tap Interact
  (if (<= (Variables|Default|GetCurrentTime) (Variables|Default|GetDelicateSwitchTime))
    (bind _output_get (Variables|Default|SetDelicateModeOn (not (Variables|Default|GetDelicateModeOn))))
    ;[1 1 1] Debug
    (Development|PrintText (Utilities|Text|FormatText "DelicateMode: {d}" _output_get))))

(fn ConstructionScript
  (|CallParentFunction))

(fn CanbeProcessed
  (for _array_element (Variables|Default|GetPlacedObjects)
    (bind _asbp_laundry_item (Utilities|Casting|CastToBP_LaundryItem _array_element))
    (return (Utilities|IsValid _asbp_laundry_item))))