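; BP_LaundryItem is a grabbable laundry piece whose mesh material follows its color (white, red, green or blue), applied at construction or through SetColor.
; Grab removes physics, then either hands the item to the player or passes it to the object already held via AddItemMessage.
; CanBeGrabbed allows pickup with empty hands or while holding a BP_Basket with free space.
; A food-state CanBeSliced check is also present.
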(event Custom|SetColor
  (params (Color :type BPE_ColorEnum%20Enum :default "NewEnumerator0"))
  (bind _output_get (Variables|Default|SetColor Color))
  (Rendering|Material|SetMaterial (Variables|Character|GetMesh) 0 (Utilities|Select :Index _output_get :NewEnumerator0 "/Engine/BasicShapes/BasicShapeMaterial.BasicShapeMaterial" :NewEnumerator1 "/AnimationSharing/AnimSharingRed.AnimSharingRed" :NewEnumerator2 "/AnimationSharing/AnimSharingGreen.AnimSharingGreen" :NewEnumerator3 "/AnimationSharing/AnimSharingBlue.AnimSharingBlue")))

(event EventBeginPlay
  (|CallParentFunction) ; This node is disabled and will not be called.\nDrag off pins to build functionality.
)

(event Collision|EventActorBeginOverlap
  (params (OtherActor :type Actor%20Object%20Reference))
  (|CallParentFunction OtherActor) ; This node is disabled and will not be called.\nDrag off pins to build functionality.
)

(event EventTick
  (params (DeltaSeconds :type Float%20%28single-precision%29))
  (|CallParentFunction DeltaSeconds) ; This node is disabled and will not be called.\nDrag off pins to build functionality.
)

(event EventGrab
  (params (Player :type BP%20Character%20Object%20Reference))
  (bind (_returnvalue _grabbedobject) (Default|GetGrabbedObject Player))
  (CallFunction|RemovePhysics)
  (if _returnvalue
    (Class|BPIBasket|AddItem(Message) _grabbedobject self)
    (else
      (Default|Grab Player self))))

(fn ConstructionScript
  (CallFunction|SetColor (Variables|Default|GetColor))
  (|CallParentFunction))

(fn CanbeSliced
  (return (and (Variables|Default|GetIsSlicable) (Utilities|Select :Index (Utilities|Enum|ByteToEnumBPE_FoodItemStates) :NewEnumerator0 true :NewEnumerator1 true :NewEnumerator2 false))))

(fn CanbeGrabbed
  (params (Player :type BP%20Character%20Object%20Reference))
  (bind (_returnvalue _grabbedobject) (Default|GetGrabbedObject Player))
  (if (not _returnvalue)
    (return true)
    (else
      (bind _asbp_basket (Utilities|Casting|CastToBP_Basket _grabbedobject)
        (:then
          (return (Default|HasPlace _asbp_basket)))
        (:CastFailed
          (return false))))))