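; BP_Countertop is an interactable counter where players place and pick up items, stored as a last-in, first-out list.
; Grab/Drop takes the top item if hands are empty or it allows grabbing while holding; otherwise it places held items of the allowed class up to a limit.
; When full, a held laundry item goes into a basket on top.
; Placing attaches the object to ObjectPlace and calls MoveComponentTo.
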(event Custom|Grab
  (params (Player :type BP%20Character%20Object%20Reference))
  ;[0.05 0.05 0.05] Grab
  (bind _output (CallFunction|GetLastObject))
  (Utilities|IsValid _output
    (:Is%20Valid
      (Default|Grab Player _output)
      (Utilities|Array|RemoveItem (Variables|Default|GetPlacedObjects) _output))))

(event Custom|Place
  (params (Player :type BP%20Character%20Object%20Reference) (ObjectToPlace :type BP%20Grabbable%20Object%20Reference))
  ;[0.05 0.05 0.05] Place
  (Utilities|Array|Add (Variables|Default|GetPlacedObjects) ObjectToPlace)
  (bind _output (CallFunction|GetLastObject))
  (Transformation|AttachComponentToComponent _output (Variables|Default|GetObjectPlace) "None" "KeepWorld" "KeepWorld" "KeepWorld" true)
  (bind _output_2 (CallFunction|GetLastObject))
  (Components|MoveComponentTo (Variables|/Script/Engine.Actor|GetRootComponent _output_2) "0, 0, 0" "0, 0, 0" false false 0.2 false)
  (Variables|/Game/_Gameplay_Albie/Blueprints/BP_Character.BP_Character_C|SetGrabbedObject Player 0))

(event EventGrab/Drop
  (params (Player :type BP%20Character%20Object%20Reference))
  (bind (_returnvalue _grabbedobject) (Default|GetGrabbedObject Player))
  ;[0.05 0.05 0.05] Grab/Drop
  ;;[0.05 0.05 0.05] Is player holding item
  (if _returnvalue
    ;;[0.05 0.05 0.05] Is there an item already here
    (bind _output (CallFunction|GetLastObject))
    (Utilities|IsValid _output
      (:Is%20Valid
        ;;[0.05 0.05 0.05] Can the item still be grabbed
        (if (Default|CanbeGrabbed _output Player)
          ;;[0.05 0.05 0.05] Grab item when holding basket
          (bind _output_2 (CallFunction|GetLastObject))
          (Default|Grab _output_2 Player)
          (Utilities|Array|RemoveItem (Variables|Default|GetPlacedObjects) _output_2)
          (else
            ;;[0.05 0.05 0.05] Place item on countertop
            ;;;[0.05 0.05 0.05] Check allowed class type
            (if (Utilities|ClassIsChildOf (Utilities|GetClass _grabbedobject) (Variables|Default|GetAllowedItemClass)) :!label _label
              ;;;[0.05 0.05 0.05] Check if space
              (if (< (Utilities|Array|Length (Variables|Default|GetPlacedObjects)) (Variables|Default|GetMaxObjects))
                (CallFunction|Place Player _grabbedobject)
                (else
                  ;[0.05 0.05 0.05] Add laundry item from hand to basket on counter
                  (bind _output_3 (CallFunction|GetLastObject))
                  (if (and (Utilities|ClassIsChildOf (Utilities|GetClass _output_3) "/Game/_Gameplay_Albie/Blueprints/Interactable/Kitchenware/BP_Basket.BP_Basket_C") (Utilities|ClassIsChildOf (Utilities|GetClass _grabbedobject) "/Game/_Gameplay_Albie/Blueprints/Interactable/BP_LaundryItem.BP_LaundryItem_C"))
                    (bind _asbp_laundry_item (Utilities|Casting|CastToBP_LaundryItem _grabbedobject))
                    (Class|BPIBasket|AddItem(Message) _output_3 _asbp_laundry_item)
                    (Variables|/Game/_Gameplay_Albie/Blueprints/BP_Character.BP_Character_C|SetGrabbedObject Player 0))))))))
      (:Is%20Not%20Valid
        (goto _label)))
    (else
      ;;[0.05 0.05 0.05] Grab item from countertop
      (CallFunction|Grab Player))))

(fn ConstructionScript)

(fn GetLastObject
  (bind _placedobjects (Variables|Default|GetPlacedObjects))
  (return (Utilities|Array|Get(acopy) _placedobjects (Utilities|Array|LastIndex _placedobjects))))