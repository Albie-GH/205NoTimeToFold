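; BP_BasketStand is an interactable stand that holds a vertical stack of laundry baskets for players to take.
; On BeginPlay it spawns the baskets without physics, attaches them at ObjectPlace and tracks them in PlacedObjects.
; Interacting while holding clean laundry adds it to the last basket and grabs, dirty laundry does nothing, and other cases use parent grab/drop.
; The Place override accepts only empty baskets back onto the stand.
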(event EventBeginPlay
  (CallFunction|InitBaskets))

(event EventPlace
  (params (Player :type BP%20Character%20Object%20Reference) (ObjectToPlace :type BP%20Grabbable%20Object%20Reference))
  ;[0.05 0.05 0.05] Only place empty baskets back on stand
  (bind _asbp_basket (Utilities|Casting|CastToBP_Basket ObjectToPlace))
  (if (Utilities|Array|IsEmpty (Variables|/Game/_Gameplay_Albie/Blueprints/Interactable/Grabbables/BP_Basket.BP_Basket_C|GetItems _asbp_basket))
    (|CallParentFunction Player ObjectToPlace)))

(event EventGrab/Drop
  (params (Player :type BP%20Character%20Object%20Reference))
  (bind _asbp_laundry_item (Utilities|Casting|CastToBP_LaundryItem (.GrabbedObject (Default|GetGrabbedObject Player)))
    (:then
      (bind _isclean (Class|BPILaundryItem|IsClean(Message) _asbp_laundry_item))
      (if _isclean
        (bind _output (CallFunction|GetLastObject))
        (Class|BPIBasket|AddItem(Message) _output _asbp_laundry_item)
        (CallFunction|Grab Player)))
    (:CastFailed
      (|CallParentFunction Player))))

(event EventGrab
  (params (Player :type BP%20Character%20Object%20Reference))
  (|CallParentFunction Player))

(fn ConstructionScript
  (|CallParentFunction))

(fn InitBaskets
  (bind _objectplace (Variables|Default|GetObjectPlace))
  (bind _returnvalue (Transformation|GetWorldLocation _objectplace))
  (for _index (range 1 (Variables|Default|GetMaxObjects))
    (bind _returnvalue_2 (Game|SpawnActorfromClass "/Game/_Gameplay_Albie/Blueprints/Interactable/Grabbables/BP_Basket.BP_Basket_C" (Math|Transform|MakeTransform (Math|Vector|MakeVector (.x _returnvalue) (.y _returnvalue) (+ (.z _returnvalue) (* (- _index 1) (Variables|Default|GetBasketHeight))))) "Undefined" "MultiplyWithRoot" 0 0))
    (Default|RemovePhysics _returnvalue_2)
    (Transformation|AttachComponentToComponent _returnvalue_2 (Variables|Default|GetObjectPlace) "None" "KeepWorld" "KeepWorld" "KeepWorld" true)
    (Utilities|Array|Add (Variables|Default|GetPlacedObjects) _returnvalue_2)))