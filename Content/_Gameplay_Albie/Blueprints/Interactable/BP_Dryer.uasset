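; BP_Dryer is an interactable laundry machine that updates the condition of placed BP_LaundryItems when its cycle finishes.
; FinishProcess adds damage for whites mixed with other colors, delicates run without delicate mode and air-dry-only items, which shrink.
; It also clears each item's wet and folded flags and refreshes its mesh state before calling the parent.
; Grab/drop passes to the parent only while the dryer is inactive.
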(event Custom|HandleTornState
  (params (Laundry%20Item :type BP%20Laundry%20Item%20Object%20Reference))
  ;[0.05 0.05 0.05] Handle damage states
  (if (Variables|/Game/_Gameplay_Albie/Blueprints/Interactable/Grabbables/BP_LaundryItem.BP_LaundryItem_C|GetIsDelicate Laundry%20Item)
    (if (not (Variables|Default|GetDelicateModeOn))
      (Utilities|Array|AddUnique (Variables|/Game/_Gameplay_Albie/Blueprints/Interactable/Grabbables/BP_LaundryItem.BP_LaundryItem_C|GetDamage Laundry%20Item) "NewEnumerator1"))))

(event Custom|HandleWet
  (params (LaundryItem :type BP%20Laundry%20Item%20Object%20Reference))
  ;[0.05 0.05 0.05] Handle wet state
  (Variables|/Game/_Gameplay_Albie/Blueprints/Interactable/Grabbables/BP_LaundryItem.BP_LaundryItem_C|SetIsWet LaundryItem false))

(event Custom|HandleShrunkState
  (params (LaundryItem :type BP%20Laundry%20Item%20Object%20Reference))
  ;[0.05 0.05 0.05] Handle damage states
  (if (Variables|/Game/_Gameplay_Albie/Blueprints/Interactable/Grabbables/BP_LaundryItem.BP_LaundryItem_C|GetAirDryOnly LaundryItem)
    (Utilities|Array|AddUnique (Variables|/Game/_Gameplay_Albie/Blueprints/Interactable/Grabbables/BP_LaundryItem.BP_LaundryItem_C|GetDamage LaundryItem) "NewEnumerator0")))

(event Custom|HandleWhites
  (params (LaundryItem :type BP%20Laundry%20Item%20Object%20Reference))
  ;[0.05 0.05 0.05] Handle whites
  (for _array_element (Variables|Default|GetPlacedObjects)
    (bind _asbp_laundry_item (Utilities|Casting|CastToBP_LaundryItem _array_element))
    (if (Utilities|Enum|NotEqual(Enum) (Variables|/Game/_Gameplay_Albie/Blueprints/Interactable/Grabbables/BP_LaundryItem.BP_LaundryItem_C|GetColor _asbp_laundry_item) "NewEnumerator0")
      (Utilities|Array|AddUnique (Variables|/Game/_Gameplay_Albie/Blueprints/Interactable/Grabbables/BP_LaundryItem.BP_LaundryItem_C|GetDamage LaundryItem) "NewEnumerator2"))))

(event Custom|HandleFold
  (params (Laundry%20Item :type BP%20Laundry%20Item%20Object%20Reference))
  ;[0.05 0.05 0.05] Handle fold state
  (Variables|/Game/_Gameplay_Albie/Blueprints/Interactable/Grabbables/BP_LaundryItem.BP_LaundryItem_C|SetIsFolded Laundry%20Item false))

(event EventGrab/Drop
  (params (Player :type BP%20Character%20Object%20Reference))
  ;[0.05 0.05 0.05] Grab/Drop Override
  (if (not (Variables|Default|GetIsActive))
    (|CallParentFunction Player)))

(event EventFinishProcess
  ;[0.05 0.05 0.05] Adjust laundry item after washing is finished
  (for _array_element (Variables|Default|GetPlacedObjects)
    (bind _asbp_laundry_item (Utilities|Casting|CastToBP_LaundryItem _array_element))
    (if (Utilities|Enum|Equal(Enum) (Variables|/Game/_Gameplay_Albie/Blueprints/Interactable/Grabbables/BP_LaundryItem.BP_LaundryItem_C|GetColor _asbp_laundry_item) "NewEnumerator0")
      (CallFunction|HandleWhites _asbp_laundry_item))
    (CallFunction|HandleTornState _asbp_laundry_item)
    (CallFunction|HandleShrunkState _asbp_laundry_item)
    (CallFunction|HandleWet _asbp_laundry_item)
    (CallFunction|HandleFold _asbp_laundry_item)
    (Default|UpdateMeshState _asbp_laundry_item))
  (|CallParentFunction))

(fn ConstructionScript
  (|CallParentFunction))