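; BP_Counter is an interactable counter that holds grabbable items on its surface at the ObjectPlace component.
; SpawnOnCounter places a passed-in laundry bag item (noted as a test path), or otherwise spawns a BP_Grabbable from SpawnActorClass.
; Either item has physics removed, attaches to ObjectPlace, is raised by its root mesh's bounding-sphere radius, and joins the PlacedObjects list.
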(fn ConstructionScript
  (|CallParentFunction))

(fn SpawnonCounter
  (params (LaundryBagItem :type BP%20Laundry%20Bag%20Object%20Reference))
  (bind _spawnactorclass (Variables|Default|GetSpawnActorClass))
  ;[1 1 1] For LaundryBag test
  (if (Utilities|IsValid LaundryBagItem)
    (Default|RemovePhysics LaundryBagItem)
    (Transformation|AttachComponentToComponent LaundryBagItem (Variables|Default|GetObjectPlace) "None" "KeepWorld" "KeepWorld" "KeepWorld" true)
    (bind _asstatic_mesh_component (Utilities|Casting|CastToStaticMeshComponent (Variables|/Script/Engine.Actor|GetRootComponent LaundryBagItem)))
    (Transformation|SetActorRelativeLocation LaundryBagItem (Math|Vector|MakeVector 0.0 0.0 (.SphereRadius (Collision|GetComponentBounds _asstatic_mesh_component))))
    (Utilities|Array|Add (Variables|Default|GetPlacedObjects) LaundryBagItem)
    (elif (Utilities|IsValidClass _spawnactorclass)
      (bind _returnvalue (Game|SpawnActorfromClass _spawnactorclass (Math|Transform|MakeTransform (Transformation|GetWorldLocation (Variables|Default|GetObjectPlace))) "Undefined" "MultiplyWithRoot" 0 0))
      (bind _asbp_grabbable (Utilities|Casting|CastToBP_Grabbable _returnvalue))
      (Default|RemovePhysics _asbp_grabbable)
      (Transformation|AttachComponentToComponent _asbp_grabbable (Variables|Default|GetObjectPlace) "None" "KeepWorld" "KeepWorld" "KeepWorld" true)
      (bind _asstatic_mesh_component_2 (Utilities|Casting|CastToStaticMeshComponent (Variables|/Script/Engine.Actor|GetRootComponent _asbp_grabbable)))
      (Transformation|SetActorRelativeLocation _asbp_grabbable (Math|Vector|MakeVector 0.0 0.0 (.SphereRadius (Collision|GetComponentBounds _asstatic_mesh_component_2))))
      (Utilities|Array|Add (Variables|Default|GetPlacedObjects) _asbp_grabbable))))