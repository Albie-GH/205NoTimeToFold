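; Base interactable Blueprint for stations that process placed objects over time and show progress on a widget bar.
; ProcessItems resets the timer and sets total time from a base time plus extra time per additional placed object.
; Each UpdateProgress call advances time by a fixed step, updates the temporary bar with a hardcoded rotation, and triggers FinishProcess when complete.
; FinishProcess resets progress and hides the bar.
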(event Custom|ProcessItems
  ;[0.05 0.05 0.05] Process Items
  (Variables|Default|SetCurrentTime 0.0)
  (Variables|Default|SetTotalTime (+ (* (- (Utilities|Array|Length (Variables|Default|GetPlacedObjects)) 1) (Variables|Default|GetExtraItemTime)) (Variables|Default|GetBaseTime))))

(event Custom|FinishProcess
  ;[0.05 0.05 0.05] Finish Process
  (Variables|Default|SetProgress 0.0)
  ;;[1 1 1] Again, temporary
  (Rendering|SetVisibility (Variables|Default|GetProgressBar) false false))

(event Custom|UpdateProgress
  (bind _progressbar (Variables|Default|GetProgressBar))
  ;[0.05 0.05 0.05] Update Progress
  (Variables|Default|SetCurrentTime (+ (Variables|Default|GetCurrentTime) 0.1))
  (bind _output_get (Variables|Default|SetProgress (* (/ (Variables|Default|GetCurrentTime) (Variables|Default|GetTotalTime)) 1e+02)))
  ;;[1 1 1] Progress Bar - Temporary
  (Rendering|SetVisibility _progressbar true false)
  (bind _aswb_progress_bar (Utilities|Casting|CastToWB_ProgressBar (UserInterface|GetWidget _progressbar)))
  (Progress|SetPercent (Variables|/Game/_Gameplay_Albie/Blueprints/WB_ProgressBar.WB_ProgressBar_C|GetItemProgress _aswb_progress_bar) (/ (Math|Float|Clamp(Float) _output_get 0.0 1e+02) 1e+02))
  ;;;[1 1 1] May have hardcoded some values here
  (Transformation|SetWorldRotation (Variables|Default|GetProgressBar) "120.000000,0.000000,180.000000" false false)
  (if (>= (Variables|Default|GetProgress) 1e+02)
    (CallFunction|FinishProcess)))

(fn ConstructionScript
  (|CallParentFunction))