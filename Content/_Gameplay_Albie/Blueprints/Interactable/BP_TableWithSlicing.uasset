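; Slicing table interactable where a player cuts a placed food item over time, extending a parent table's grab/drop behavior.
; Interact checks that the food can be sliced, changes its state and marks the player as interacting.
; Tick advances progress at a constant slicing speed, updates a widget progress bar, then ends the interaction and sets the food's next state.
; Grab/drop works only at zero or full progress and resets it.
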(event EventTick
  (params (DeltaSeconds :type Float%20%28single-precision%29))
  (|CallParentFunction DeltaSeconds)
  (if (Variables|Default|GetIsInteracting)
    (bind _output_get (Variables|Default|SetProgress (Math|Interpolation|FInterptoConstant (Variables|Default|GetProgress) 1.0 DeltaSeconds (Variables|Settings|GetSlicingSpeed))))
    (Development|PrintString (Utilities|String|ToString(Float) _output_get) true true "(R=0.000000,G=0.660000,B=1.000000,A=1.000000)" DeltaSeconds)
    ;[1 1 1] Progress Bar - Not From Tutorial
    (Rendering|SetVisibility (Variables|Default|GetProgressBarWidget) true false)
    (bind _aswb_progress_bar (Utilities|Casting|CastToWB_ProgressBar (UserInterface|GetWidget (Variables|Default|GetProgressBarWidget))))
    (Progress|SetPercent (Variables|/Game/_Gameplay_Albie/Blueprints/WB_ProgressBar.WB_ProgressBar_C|GetItemProgress _aswb_progress_bar) _output_get)
    ;;[1 1 1] May have hardcoded some values here
    (Transformation|SetWorldRotation (Variables|Default|GetProgressBarWidget) "120.000000,0.000000,180.000000" false false)
    (if (== (Variables|Default|GetProgress) 1.0)
      ;[1 1 1] This Too
      (Rendering|SetVisibility (Variables|Default|GetProgressBarWidget) false false)
      (CallFunction|StopInteraction)
      (bind _asbp_food_item (Utilities|Casting|CastToBP_FoodItem (Variables|Default|GetPlacedObject)))
      (Default|SetState _asbp_food_item "NewEnumerator2"))))

(event EventGrab/Drop
  (params (Player :type BP%20Character%20Object%20Reference))
  (if (CallFunction|CanGrabObject)
    (|CallParentFunction Player)
    (Variables|Default|SetProgress 0.0)))

(event EventInteract
  (params (player :type BP%20Character%20Object%20Reference))
  (bind _asbp_food_item (Utilities|Casting|CastToBP_FoodItem (Variables|Default|GetPlacedObject)))
  (if (Default|CanbeSliced _asbp_food_item)
    (Default|SetState _asbp_food_item "NewEnumerator1")
    (Default|SetIsInteracting player true self)
    (Variables|Default|SetInteractingPlayer player)
    (Variables|Default|SetIsInteracting true)))

(event EventStopInteraction
  (Variables|Default|SetIsInteracting false)
  (Default|SetIsInteracting (Variables|Default|GetInteractingPlayer) false)
  (Development|PrintString "Stopped interacting"))

(fn ConstructionScript
  (|CallParentFunction))

(fn CanGrabObject
  (return (or (== (Variables|Default|GetProgress) 0.0) (== (Variables|Default|GetProgress) 1.0))))