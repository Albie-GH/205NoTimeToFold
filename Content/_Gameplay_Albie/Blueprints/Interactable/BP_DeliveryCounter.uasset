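; Delivery counter interactable where a player drops a laundry basket to complete a matching active order.
; Grab/Drop scans the game state's active orders for an equal item count, striking items from a temporary copy by colour and delicate flag only.
; When that copy empties, it converts basket items to BP_DataItem objects for quality data, passes them to CompleteOrder and destroys the basket.
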(event EventGrab/Drop
  (params (Player :type BP%20Character%20Object%20Reference))
  (bind (_returnvalue _grabbedobject) (Default|GetGrabbedObject Player))
  (if _returnvalue
    (Variables|Default|SetOrderFound false)
    (bind _asbp_basket (Utilities|Casting|CastToBP_Basket _grabbedobject))
    (bind _array_element (Utilities|Array|ForEachLoopwithBreak (Variables|/Game/_Gameplay_Albie/Blueprints/BP_GameState.BP_GameState_C|GetActiveOrders (Variables|Default|GetGameState)) :!label _label)
      (:LoopBody
        ;[0.05 0.05 0.05] Temporary order to do checks
        (if (== (Utilities|Array|Length (Variables|/Game/_Gameplay_Albie/Blueprints/Data/BP_DataOrder.BP_DataOrder_C|GetOrderItems _array_element)) (Utilities|Array|Length (Variables|/Game/_Gameplay_Albie/Blueprints/Interactable/Grabbables/BP_Basket.BP_Basket_C|GetItems _asbp_basket)))
          (bind _output_get (Variables|Default|SetTempOrder (Variables|/Game/_Gameplay_Albie/Blueprints/Data/BP_DataOrder.BP_DataOrder_C|GetOrderItems _array_element)))
          (bind _array_element_2 (Utilities|Array|ForEachLoopwithBreak (Variables|/Game/_Gameplay_Albie/Blueprints/Data/BP_DataOrder.BP_DataOrder_C|GetOrderItems _array_element))
            (:LoopBody
              ;[0.05 0.05 0.05] Compare and remove items from temp order
              (for _array_element_3 (Variables|/Game/_Gameplay_Albie/Blueprints/Interactable/Grabbables/BP_Basket.BP_Basket_C|GetItems _asbp_basket)
                (if (and (Utilities|Enum|Equal(Enum) (Variables|/Game/_Gameplay_Albie/Blueprints/Interactable/Grabbables/BP_LaundryItem.BP_LaundryItem_C|GetColor _array_element_3) (Variables|/Game/_Gameplay_Albie/Blueprints/Data/BP_DataItem.BP_DataItem_C|GetColor _array_element_2)) (== (Variables|/Game/_Gameplay_Albie/Blueprints/Interactable/Grabbables/BP_LaundryItem.BP_LaundryItem_C|GetIsDelicate _array_element_3) (Variables|/Game/_Gameplay_Albie/Blueprints/Data/BP_DataItem.BP_DataItem_C|GetIsDelicate _array_element_2)))
                  (Utilities|Array|RemoveItem _output_get _array_element_2))))
            (:Completed
              ;[0.05 0.05 0.05] If temp order is empty - complete order
              (if (Utilities|Array|IsEmpty _output_get)
                (for _array_element_4 (Variables|/Game/_Gameplay_Albie/Blueprints/Interactable/Grabbables/BP_Basket.BP_Basket_C|GetItems _asbp_basket)
                  (bind _laundrydataitem (CallFunction|ConverttoDataItem (Variables|/Game/_Gameplay_Albie/Blueprints/Interactable/Grabbables/BP_LaundryItem.BP_LaundryItem_C|GetColor _array_element_4) (Variables|/Game/_Gameplay_Albie/Blueprints/Interactable/Grabbables/BP_LaundryItem.BP_LaundryItem_C|GetIsDelicate _array_element_4) (Variables|/Game/_Gameplay_Albie/Blueprints/Interactable/Grabbables/BP_LaundryItem.BP_LaundryItem_C|GetAirDryOnly _array_element_4) (Variables|/Game/_Gameplay_Albie/Blueprints/Interactable/Grabbables/BP_LaundryItem.BP_LaundryItem_C|GetIsStained _array_element_4) (Variables|/Game/_Gameplay_Albie/Blueprints/Interactable/Grabbables/BP_LaundryItem.BP_LaundryItem_C|GetWashState _array_element_4) (Variables|/Game/_Gameplay_Albie/Blueprints/Interactable/Grabbables/BP_LaundryItem.BP_LaundryItem_C|GetDamage _array_element_4) (Variables|/Game/_Gameplay_Albie/Blueprints/Interactable/Grabbables/BP_LaundryItem.BP_LaundryItem_C|GetIsFolded _array_element_4)))
                  (Utilities|Array|Add (Variables|Default|GetCompleteOrderQuality) _laundrydataitem))
                (Default|CompleteOrder (Variables|Default|GetGameState) _array_element (Variables|Default|GetCompleteOrderQuality))
                (bind _asbp_basket_2 (Utilities|Casting|CastToBP_Basket _grabbedobject))
                (Default|DestroySelf _asbp_basket_2)
                (Variables|/Game/_Gameplay_Albie/Blueprints/BP_Character.BP_Character_C|SetGrabbedObject Player 0)
                (Variables|Default|SetOrderFound true)
                (goto _label Break)))))))))

(event EventBeginPlay
  (bind _asbp_game_state (Utilities|Casting|CastToBP_GameState (Game|GetGameState)))
  (Variables|Default|SetGameState _asbp_game_state))

(fn ConstructionScript
  (|CallParentFunction))

(fn ConverttoDataItem
  (params (Color :type BPE_ColorEnum%20Enum :default "NewEnumerator0") (IsDelicate :type Boolean) (AirDryOnly :type Boolean) (IsStained :type Boolean) (WashState :type BPE_WashedEnum%20Enum :default "NewEnumerator1") (Damage :type Array%20of%20BPE_DamageEnum%20Enums :default "NewEnumerator0") (IsFolded :type Boolean))
  (bind _returnvalue (Game|ConstructObjectfromClass "/Game/_Gameplay_Albie/Blueprints/Data/BP_DataItem.BP_DataItem_C" Color IsDelicate AirDryOnly IsStained WashState Damage IsFolded))
  (return _returnvalue))