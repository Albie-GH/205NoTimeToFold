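; Food dispenser interactable that hands a newly spawned BP_FoodItem to an empty-handed player.
; Grab/Drop defers to the parent behavior when a placed object can be grabbed, or when the box is empty and the player holds something.
; With nothing placed or held, it spawns the item at the box's transform and immediately calls GrabDrop on it for that player.
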(event EventGrab/Drop
  (params (Player :type BP%20Character%20Object%20Reference))
  (bind _placedobject (Variables|Default|GetPlacedObject)
    (:then
      (if (Default|CanbeGrabbed _placedobject Player)
        (|CallParentFunction Player :!label _label)))
    (:else
      (if (.ReturnValue (Default|GetGrabbedObject Player))
        (goto _label)
        (else
          (bind _returnvalue (Game|SpawnActorfromClass "/Game/_Gameplay_Albie/Blueprints/Interactable/BP_FoodItem.BP_FoodItem_C" (Transformation|GetActorTransform) "Undefined" "MultiplyWithRoot" 0 true 0))
          (Default|Grab/Drop _returnvalue Player))))))

(fn ConstructionScript
  (|CallParentFunction))