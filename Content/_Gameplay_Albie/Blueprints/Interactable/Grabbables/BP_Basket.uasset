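; BP_Basket is a grabbable laundry basket that collects clean, dry laundry items.
; Grabbing it runs AddItemFromCharacter on the player's held item before the parent grab, while CanBeGrabbed allows only empty-handed players.
; AddItem attaches items to ItemPlace, slides them into a stack offset by mesh bounds and count, then updates icons.
; HasPlace reports spare capacity, and DestroySelf destroys the contents with the basket.
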(event EventGrab
  (params (Player :type BP%20Character%20Object%20Reference))
  (CallFunction|AddItemfromCharacter Player)
  (|CallParentFunction Player))

(event EventAddItem
  (params (LaundryItem :type BP%20Laundry%20Item%20Object%20Reference))
  (bind _items (Variables|Default|GetItems))
  (bind _rootcomponent (Variables|/Script/Engine.Actor|GetRootComponent LaundryItem))
  (Utilities|Array|Add _items LaundryItem)
  (Default|HideIconDetails LaundryItem)
  (Transformation|AttachComponentToComponent LaundryItem (Variables|Default|GetItemPlace) "None" "KeepWorld" "KeepWorld" "KeepWorld" true)
  ;[1 1 1] Debug
  (Development|PrintText (Utilities|Text|FormatText "In Basket: {num}" (Utilities|Array|Length _items)))
  (bind _asstatic_mesh_component (Utilities|Casting|CastToStaticMeshComponent _rootcomponent))
  (Components|MoveComponentTo _rootcomponent (Math|Vector|MakeVector 0.0 0.0 (* (* (.z (.BoxExtent (Collision|GetComponentBounds _asstatic_mesh_component))) 2.0) (- (Utilities|Array|Length (Variables|Default|GetItems)) 1))) "0, 0, 0" false false 0.2 false)
  (CallFunction|UpdateIcons))

(fn ConstructionScript
  (|CallParentFunction))

(fn HasPlace
  (return (< (Utilities|Array|Length (Variables|Default|GetItems)) (Variables|Default|GetMaxItemsCount))))

(fn CanbeGrabbed
  (params (Player :type BP%20Character%20Object%20Reference))
  (if (.ReturnValue (Default|GetGrabbedObject Player))
    (return false)
    (else
      (return true))))

(fn AddItemfromCharacter
  (params (Character :type BP%20Character%20Object%20Reference))
  (bind (_returnvalue _grabbedobject) (Default|GetGrabbedObject Character))
  (if _returnvalue
    (bind _asbp_laundry_item (Utilities|Casting|CastToBP_LaundryItem _grabbedobject))
    (bind _isclean (Default|IsClean _asbp_laundry_item))
    (bind _isdry (Default|IsDry _asbp_laundry_item))
    (if (and _isdry _isclean)
      (CallFunction|AddItem _asbp_laundry_item))))

(fn DestroySelf
  (for _array_element (Variables|Default|GetItems)
    (Actor|DestroyActor _array_element))
  (Actor|DestroyActor))