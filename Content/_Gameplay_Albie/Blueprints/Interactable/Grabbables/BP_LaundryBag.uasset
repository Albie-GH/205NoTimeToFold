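; Grabbable laundry bag that holds a stack of laundry items, offering functions to read and remove the last one.
; InitItems, called on BeginPlay, spawns BP_LaundryItems from an array of item data, copying color and care flags, then attaches them without physics at ItemPlace.
; IsEmpty also destroys the bag when no items remain.
; A random item generator remains in InitItems but never runs.
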(event EventGrab/Drop
  (params (Player :type BP%20Character%20Object%20Reference))
  (|CallParentFunction Player))

(event EventBeginPlay
  (CallFunction|InitItems)
  (|CallParentFunction))

(fn ConstructionScript
  (|CallParentFunction))

(fn InitItems
  (params (ItemsToInit :type Array%20of%20BP%20Data%20Item%20Object%20References))
  ;[0.05 0.05 0.05] Initialize bag with BP_LaundryItems from array of BP_DataItems
  (if (Utilities|Array|IsNotEmpty ItemsToInit)
    (for _array_element ItemsToInit
      (bind _returnvalue (Game|SpawnActorfromClass "/Game/_Gameplay_Albie/Blueprints/Interactable/Grabbables/BP_LaundryItem.BP_LaundryItem_C" (Math|Conversions|ToTransform(Vector) (Transformation|GetWorldLocation (Variables|Default|GetItemPlace))) "Undefined" "MultiplyWithRoot" 0 0))
      (Default|SetColor _returnvalue (Variables|/Game/_Gameplay_Albie/Blueprints/BP_DataItem.BP_DataItem_C|GetColor _array_element))
      (Variables|/Game/_Gameplay_Albie/Blueprints/Interactable/Grabbables/BP_LaundryItem.BP_LaundryItem_C|SetIsDelicate _returnvalue (Variables|/Game/_Gameplay_Albie/Blueprints/BP_DataItem.BP_DataItem_C|GetIsDelicate _array_element))
      (Variables|/Game/_Gameplay_Albie/Blueprints/Interactable/Grabbables/BP_LaundryItem.BP_LaundryItem_C|SetAirDryOnly _returnvalue (Variables|/Game/_Gameplay_Albie/Blueprints/BP_DataItem.BP_DataItem_C|GetAirDryOnly _array_element))
      (Variables|/Game/_Gameplay_Albie/Blueprints/Interactable/Grabbables/BP_LaundryItem.BP_LaundryItem_C|SetIsStained _returnvalue (Variables|/Game/_Gameplay_Albie/Blueprints/BP_DataItem.BP_DataItem_C|GetIsStained _array_element))
      (Default|RemovePhysics _returnvalue)
      (Transformation|AttachComponentToComponent _returnvalue (Variables|Default|GetItemPlace) "None" "KeepWorld" "KeepWorld" "KeepWorld" true)
      (Utilities|Array|Add (Variables|Contents|GetItems) _returnvalue))))

(fn GetLastItem
  (bind _items (Variables|Contents|GetItems))
  (return (Utilities|Array|Get(acopy) _items (Utilities|Array|LastIndex _items))))

(fn IsEmpty
  (if (Utilities|Array|IsEmpty (Variables|Contents|GetItems))
    (Actor|DestroyActor)
    (return true)
    (else
      (return false))))

(fn RemoveLastItem
  (bind _items (Variables|Contents|GetItems))
  (bind _returnvalue (Utilities|Array|LastIndex _items))
  (Utilities|Array|RemoveIndex _items _returnvalue)
  ;[1 1 1] Debug
  (Development|PrintText (Utilities|Text|FormatText "In Bag: {n}" (+ _returnvalue 1)))
  (return))