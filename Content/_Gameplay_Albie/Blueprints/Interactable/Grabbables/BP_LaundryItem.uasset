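; BP_LaundryItem is a grabbable laundry item with color, wash, stain, wet, damage, delicate and folded state.
; SetMeshState looks up its mesh in the game state's map by color, wash, wet and fold, falling back to a cube.
; Empty-handed players can grab any item, while basket holders can add only clean items if space remains.
; Grab removes physics, then either messages the held object or attaches to the player and prints debug state.
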(event EventBeginPlay
  (bind _asbp_game_state (Utilities|Casting|CastToBP_GameState (Game|GetGameState)))
  (CallFunction|SetMeshState (Variables|Default|GetColor) "NewEnumerator1" false false false (Variables|/Game/_Gameplay_Albie/Blueprints/BP_GameState.BP_GameState_C|GetLaundryMeshMap _asbp_game_state))
  (|CallParentFunction))

(event EventGrab
  (params (Player :type BP%20Character%20Object%20Reference))
  (bind (_returnvalue _grabbedobject) (Default|GetGrabbedObject Player))
  (bind _damage (Variables|Default|GetDamage))
  ;[0.05 0.05 0.05] Grab item to hands or basket
  (CallFunction|RemovePhysics)
  (if _returnvalue
    (Class|BPIBasket|AddItem(Message) _grabbedobject self)
    (else
      (Default|Grab Player self)
      ;[1 1 1] Print on pick up off ground
      (if (Utilities|Array|IsEmpty _damage)
        (Variables|Default|SetDamageString "No")
        (else
          (for _array_element _damage
            (Variables|Default|SetDamageString (Utilities|String|Append "" (Utilities|String|EnumtoString _array_element))))))
      (Development|PrintText (Utilities|Text|FormatText "WashState {w} 
Stain {s} 
Wet {wet} 
Damage {d} 
Delicate {del} 
Folded {f}" (Utilities|Text|ToText(String) (Utilities|String|EnumtoString (Variables|Default|GetWashState))) (Variables|Default|GetIsStained) (Variables|Default|GetIsWet) (Variables|Default|GetDamageString) (Variables|Default|GetIsDelicate) (Variables|Default|GetIsFolded))))))

(event EventGrab/Drop
  (params (Player :type BP%20Character%20Object%20Reference))
  ;[0.05 0.05 0.05] Grab/Drop Override
  (if (CallFunction|CanbeGrabbed Player)
    (|CallParentFunction Player)))

(fn ConstructionScript
  (|CallParentFunction))

(fn CanbeWashed
  (return (Utilities|Select :Index (Variables|Default|GetWashState) :NewEnumerator1 true :NewEnumerator2 true :NewEnumerator3 false)))

(fn CanbeGrabbed
  (params (Player :type BP%20Character%20Object%20Reference))
  (bind (_returnvalue _grabbedobject) (Default|GetGrabbedObject Player))
  (if (not _returnvalue)
    ;[0.05 0.05 0.05] Player not holding anything
    (return true)
    (else
      (bind _asbp_basket (Utilities|Casting|CastToBP_Basket _grabbedobject)
        (:then
          (if (Default|HasPlace _asbp_basket)
            (bind _isclean (CallFunction|IsClean))
            (if _isclean
              ;[0.05 0.05 0.05] Item is clean and player holding basket with enough space
              (return true)
              (else
                ;[0.05 0.05 0.05] Item not clean
                (return false)))
            (else
              ;[0.05 0.05 0.05] Player holding full basket
              (return false))))
        (:CastFailed
          ;[0.05 0.05 0.05] Player not holding basket
          (return false))))))

(fn SetMeshState
  (params (Color :type BPE_ColorEnum%20Enum :default "NewEnumerator0") (WashState :type BPE_WashedEnum%20Enum :default "NewEnumerator1") (IsStained :type Boolean) (IsWet :type Boolean) (IsFolded :type Boolean) (LaundryMeshMap :type Map%20of%20F%20Laundry%20Mesh%20Struct%20Structures%20to%20Objects))
  (bind _output_get (Variables|Default|SetColor Color))
  (if (.ReturnValue (Utilities|Map|Find LaundryMeshMap (Utilities|Struct|MakeFLaundryMeshStruct _output_get WashState IsWet IsFolded)))
    (Components|StaticMesh|SetStaticMesh (Variables|Character|GetMesh) (.Value (Utilities|Map|Find LaundryMeshMap (Utilities|Struct|MakeFLaundryMeshStruct _output_get WashState IsWet IsFolded))))
    (else
      (Components|StaticMesh|SetStaticMesh (Variables|Character|GetMesh) "/Engine/EngineMeshes/Cube.Cube"))))

(fn IsClean
  (return (Utilities|Select :Index (Variables|Default|GetWashState) :NewEnumerator1 false :NewEnumerator2 false :NewEnumerator3 true)))

(fn IsDry
  (return (not (Variables|Default|GetIsWet))))