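; BP_Container is a grabbable interactable that holds a list of items, apparently a bag.
; Grab/drop and construction defer to the parent class.
; Helper functions treat the Items array like a stack, returning or removing the last entry, with removal printing the remaining count as debug text.
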(event EventGrab/Drop
  (params (Player :type BP%20Character%20Object%20Reference))
  (|CallParentFunction Player))

(fn ConstructionScript
  (|CallParentFunction))

(fn GetLastItem
  (bind _items (Variables|Default|GetItems))
  (return (Utilities|Array|Get(acopy) _items (Utilities|Array|LastIndex _items))))

(fn RemoveLastItem
  (bind _items (Variables|Default|GetItems))
  (bind _returnvalue (Utilities|Array|LastIndex _items))
  (Utilities|Array|RemoveIndex _items _returnvalue)
  ;[1 1 1] Debug
  (Development|PrintText (Utilities|Text|FormatText "In Bag: {n}" (+ _returnvalue 1)))
  (return))