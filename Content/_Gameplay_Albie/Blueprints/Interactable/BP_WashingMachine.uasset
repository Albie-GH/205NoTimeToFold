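; Washing machine interactable that turns placed laundry items wet and unfolded, cleaning or damaging them based on additives and delicate mode.
; Interact and Grab/Drop first try loading held detergent or whitener while idle, otherwise deferring to parent behavior.
; FinishProcess updates each item: detergent cleans, except normal clothes on delicate mode; delicates are damaged without it.
; Whitener clears white discoloration, mixed colors reapply it, then additives reset and icons refresh.
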(event Custom|HandleDamageState
  (params (Laundry%20Item :type BP%20Laundry%20Item%20Object%20Reference))
  ;[0.05 0.05 0.05] Handle damage state
  (if (Variables|/Game/_Gameplay_Albie/Blueprints/Interactable/Grabbables/BP_LaundryItem.BP_LaundryItem_C|GetIsDelicate Laundry%20Item)
    (if (not (Variables|Default|GetDelicateModeOn))
      (Utilities|Array|AddUnique (Variables|/Game/_Gameplay_Albie/Blueprints/Interactable/Grabbables/BP_LaundryItem.BP_LaundryItem_C|GetDamage Laundry%20Item) "NewEnumerator1"))))

(event Custom|HandleWet
  (params (LaundryItem :type BP%20Laundry%20Item%20Object%20Reference))
  ;[0.05 0.05 0.05] Handle wet state
  (Variables|/Game/_Gameplay_Albie/Blueprints/Interactable/Grabbables/BP_LaundryItem.BP_LaundryItem_C|SetIsWet LaundryItem true))

(event Custom|HandleWashState
  (params (Laundry%20Item :type BP%20Laundry%20Item%20Object%20Reference))
  ;[0.05 0.05 0.05] Handle wash state
  (bind _isclean (Default|IsClean Laundry%20Item))
  (if (not _isclean)
    (if (Variables|Default|GetHasDetergent)
      (if (Variables|/Game/_Gameplay_Albie/Blueprints/Interactable/Grabbables/BP_LaundryItem.BP_LaundryItem_C|GetIsDelicate Laundry%20Item)
        (Variables|/Game/_Gameplay_Albie/Blueprints/Interactable/Grabbables/BP_LaundryItem.BP_LaundryItem_C|SetWashState Laundry%20Item "NewEnumerator3" :!label _label)
        (else
          ;;[0.05 0.05 0.05] Normal clothes don't get cleaned when delicate mode is on
          (if (not (Variables|Default|GetDelicateModeOn))
            (goto _label)))))))

(event Custom|HandleWhites
  (params (LaundryItem :type BP%20Laundry%20Item%20Object%20Reference))
  (bind _damage (Variables|/Game/_Gameplay_Albie/Blueprints/Interactable/Grabbables/BP_LaundryItem.BP_LaundryItem_C|GetDamage LaundryItem))
  ;[0.05 0.05 0.05] Handle whites
  ;;[0.05 0.05 0.05] Whitener
  (if (Variables|Default|GetHasWhitener)
    (if (Utilities|Array|ContainsItem _damage "NewEnumerator2")
      (Utilities|Array|RemoveItem _damage "NewEnumerator2")))
  ;;[0.05 0.05 0.05] Discolored
  (for _array_element (Variables|Default|GetPlacedObjects)
    (bind _asbp_laundry_item (Utilities|Casting|CastToBP_LaundryItem _array_element))
    (if (Utilities|Enum|NotEqual(Enum) (Variables|/Game/_Gameplay_Albie/Blueprints/Interactable/Grabbables/BP_LaundryItem.BP_LaundryItem_C|GetColor _asbp_laundry_item) "NewEnumerator0")
      (Utilities|Array|AddUnique (Variables|/Game/_Gameplay_Albie/Blueprints/Interactable/Grabbables/BP_LaundryItem.BP_LaundryItem_C|GetDamage LaundryItem) "NewEnumerator2"))))

(event Custom|HandleFold
  (params (Laundry%20Item :type BP%20Laundry%20Item%20Object%20Reference))
  ;[0.05 0.05 0.05] Handle fold state
  (Variables|/Game/_Gameplay_Albie/Blueprints/Interactable/Grabbables/BP_LaundryItem.BP_LaundryItem_C|SetIsFolded Laundry%20Item false))

(event EventInteract
  (params (player :type BP%20Character%20Object%20Reference))
  ;[0.05 0.05 0.05] Interact Override
  (bind _detergentadded (CallFunction|TryAddDetergent player))
  (if _detergentadded
    ;[1 1 1] Debug
    (Development|PrintString "Detergent added")
    (else
      (bind _whiteneradded (CallFunction|TryAddWhitener player))
      (if _whiteneradded
        (Development|PrintString "Whitener added")
        (else
          (|CallParentFunction player))))))

(event EventGrab/Drop
  (params (Player :type BP%20Character%20Object%20Reference))
  ;[0.05 0.05 0.05] Grab/Drop Override
  (bind _detergentadded (CallFunction|TryAddDetergent Player))
  (if _detergentadded
    ;[1 1 1] Debug
    (Development|PrintString "Detergent added")
    (else
      (bind _whiteneradded (CallFunction|TryAddWhitener Player))
      (if _whiteneradded
        (Development|PrintString "Whitener added")
        (elif (not (Variables|Default|GetIsActive))
          (Audio|PlaySound2D "/Game/Aedan_UI/Sounds/631887__greatsoundstube__washing-machine-door-close-gently.631887__greatsoundstube__washing-machine-door-close-gently" 1.0 1.0 0.0 0 0)
          (|CallParentFunction Player))))))

(event EventFinishProcess
  ;[0.05 0.05 0.05] Adjust laundry item after washing is finished
  (for _array_element (Variables|Default|GetPlacedObjects)
    (bind _asbp_laundry_item (Utilities|Casting|CastToBP_LaundryItem _array_element))
    (if (Utilities|Enum|Equal(Enum) (Variables|/Game/_Gameplay_Albie/Blueprints/Interactable/Grabbables/BP_LaundryItem.BP_LaundryItem_C|GetColor _asbp_laundry_item) "NewEnumerator0")
      (CallFunction|HandleWhites _asbp_laundry_item))
    (CallFunction|HandleWashState _asbp_laundry_item)
    (CallFunction|HandleDamageState _asbp_laundry_item)
    (CallFunction|HandleWet _asbp_laundry_item)
    (CallFunction|HandleFold _asbp_laundry_item)
    (Default|UpdateMeshState _asbp_laundry_item))
  (Variables|Default|SetHasDetergent false)
  (Variables|Default|SetHasWhitener false)
  (CallFunction|UpdateMachineIcons)
  (|CallParentFunction))

(fn ConstructionScript
  (|CallParentFunction))

(fn TryAddDetergent
  (params (Player :type BP%20Character%20Object%20Reference))
  (if (not (Variables|Default|GetIsActive))
    (if (not (Variables|Default|GetHasDetergent))
      (Utilities|Casting|CastToBP_Detergent (Variables|/Game/_Gameplay_Albie/Blueprints/BP_Character.BP_Character_C|GetGrabbedObject Player)
        (:then
          (Audio|PlaySound2D "/Game/Aedan_UI/Sounds/177986__lampeight__dryerdooropen.177986__lampeight__dryerdooropen" 1.0 1.0 0.0 0 0)
          (bind _output_get (Variables|Default|SetHasDetergent true))
          (CallFunction|UpdateMachineIcons)
          (return _output_get))
        (:CastFailed
          _))))
  (return false))

(fn TryAddWhitener
  (params (Player :type BP%20Character%20Object%20Reference))
  (if (not (Variables|Default|GetIsActive))
    (if (not (Variables|Default|GetHasWhitener))
      (Utilities|Casting|CastToBP_Whitener (Variables|/Game/_Gameplay_Albie/Blueprints/BP_Character.BP_Character_C|GetGrabbedObject Player)
        (:then
          (Audio|PlaySound2D "/Game/Aedan_UI/Sounds/177986__lampeight__dryerdooropen.177986__lampeight__dryerdooropen" 1.0 1.0 0.0 0 0)
          (bind _output_get (Variables|Default|SetHasWhitener true))
          (CallFunction|UpdateMachineIcons)
          (return _output_get))
        (:CastFailed
          _))))
  (return false))

(fn UpdateMachineIcons
  (|CallParentFunction)
  (Utilities|FlowControl|Sequence
    (:then_0
      (if (Variables|Default|GetHasDetergent)
        (Utilities|Array|AddUnique (Variables|Default|GetMachineIcons) "NewEnumerator2")))
    (:then_1
      (if (Variables|Default|GetHasWhitener)
        (Utilities|Array|AddUnique (Variables|Default|GetMachineIcons) "NewEnumerator3")))
    (:then_2
      (bind _aswbp_machine_icon_slots (Utilities|Casting|CastToWBP_MachineIconSlots (UserInterface|GetUserWidgetObject (Variables|Default|GetMachineIconWidget))))
      (Default|UpdateIcons _aswbp_machine_icon_slots (Variables|Default|GetMachineIcons)))))