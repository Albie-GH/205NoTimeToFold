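; BP_FoodItem is a grabbable food item that tracks a Raw, Slicing or Sliced state.
; SetState stores the state and swaps the mesh material, while CanBeSliced allows slicing only on sliceable items that are not yet Sliced.
; Grab removes physics, then passes the food to the player's held object via an AddItem message, or to empty hands.
; CanBeGrabbed requires empty hands or held BP_Kitchenware with free space.
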(event Custom|SetState
  (params (State :type BPE_FoodItemStates%20Enum :default "NewEnumerator0"))
  (bind _output_get (Variables|Default|SetState State))
  (Rendering|Material|SetMaterial (Variables|Character|GetMesh) 0 (Utilities|Select :Index _output_get :NewEnumerator0 0 :NewEnumerator1 "/DatasmithContent/Materials/AliasReference.AliasReference" :NewEnumerator2 "/DatasmithContent/Materials/FBXImporter/VRED/MetallicCarpaint.MetallicCarpaint")))

(event EventBeginPlay
  (|CallParentFunction) ; This node is disabled and will not be called.\nDrag off pins to build functionality.
)

(event Collision|EventActorBeginOverlap
  (params (OtherActor :type Actor%20Object%20Reference))
  (|CallParentFunction OtherActor) ; This node is disabled and will not be called.\nDrag off pins to build functionality.
)

(event EventTick
  (params (DeltaSeconds :type Float%20%28single-precision%29))
  (|CallParentFunction DeltaSeconds) ; This node is disabled and will not be called.\nDrag off pins to build functionality.
)

(event EventGrab
  (params (Player :type BP%20Character%20Object%20Reference))
  (bind (_returnvalue _grabbedobject) (Default|GetGrabbedObject Player))
  (CallFunction|RemovePhysics)
  (if _returnvalue
    (Class|BPIDish|AddItem(Message) _grabbedobject self)
    (else
      (Default|Grab Player self))))

(fn ConstructionScript
  (|CallParentFunction))

(fn CanbeSliced
  (return (and (Variables|Default|GetIsSlicable) (Utilities|Select :Index (Variables|Default|GetState) :NewEnumerator0 true :NewEnumerator1 true :NewEnumerator2 false))))

(fn CanbeGrabbed
  (params (Player :type BP%20Character%20Object%20Reference))
  (bind (_returnvalue _grabbedobject) (Default|GetGrabbedObject Player))
  (if (not _returnvalue)
    (return true)
    (else
      (bind _asbp_kitchenware (Utilities|Casting|CastToBP_Kitchenware _grabbedobject)
        (:then
          (return (Default|HasPlace _asbp_kitchenware)))
        (:CastFailed
          (return false))))))