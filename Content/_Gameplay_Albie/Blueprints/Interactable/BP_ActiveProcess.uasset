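; BP_ActiveProcess is an interactable processing station that works on placed laundry items while the player holds the interact button.
; Interact runs only if every placed object is a laundry item, flags the player as interacting, starts processing at zero progress and ticks progress on a looping timer.
; Releasing or finishing stops the timer and frees the player, with update and finish logic delegated to the parent class.
; Grab/drop is blocked while progress is underway.
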(event EventInteract
  (params (player :type BP%20Character%20Object%20Reference))
  ;[0.05 0.05 0.05] Interact while button is held
  (bind _canbeprocessed (CallFunction|CanbeProcessed))
  (if _canbeprocessed
    (Default|SetIsInteracting player true self)
    (Variables|Default|SetInteractingPlayer player)
    (if (== (Variables|Default|GetProgress) 0.0)
      (CallFunction|ProcessItems))
    (bind _output_get (Variables|Default|SetIsInteracting true))
    (Utilities|Time|SetTimerbyEvent (delegate EventUpdateProgress) 0.1 _output_get)))

(event EventUpdateProgress
  ;[0.05 0.05 0.05] Interact while button is held
  (|CallParentFunction))

(event EventGrab/Drop
  (params (Player :type BP%20Character%20Object%20Reference))
  ;[0.05 0.05 0.05] Grab/Drop
  ;;[0.05 0.05 0.05] Check if in middle of process before picking up
  (if (not (!= (Variables|Default|GetProgress) 0.0))
    (|CallParentFunction Player)))

(event EventFinishProcess
  ;[0.05 0.05 0.05] Finish process and stop interaction
  (CallFunction|StopInteraction)
  (|CallParentFunction))

(event EventStopInteraction
  ;[0.05 0.05 0.05] Stop interact on button release
  (Variables|Default|SetIsInteracting false)
  (Default|SetIsInteracting (Variables|Default|GetInteractingPlayer) false)
  (Development|PrintString "Stop Interaction")
  (Utilities|Time|ClearTimerbyFunctionName 0 "UpdateProgress"))

(fn ConstructionScript
  (|CallParentFunction))

(fn CanbeProcessed
  (if (Utilities|Array|IsNotEmpty (Variables|Default|GetPlacedObjects))
    (for _array_element (Variables|Default|GetPlacedObjects)
      (Utilities|Casting|CastToBP_LaundryItem _array_element
        (:CastFailed
          ;[0.05 0.05 0.05] Invalid
          (return false))))
    ;[0.05 0.05 0.05] Valid
    (return true)
    (else
      (return false))))