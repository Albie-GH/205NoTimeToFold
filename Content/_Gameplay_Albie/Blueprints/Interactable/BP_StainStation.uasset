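; BP_StainStation is a processing station that removes stains from placed laundry items.
; CanBeProcessed extends the parent check, passing only if every placed object is a stained BP_LaundryItem.
; FinishProcess clears each item's stained and folded flags, calling the parent's FinishProcess inside the loop, once per item.
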(event EventFinishProcess
  ;[0.05 0.05 0.05] Adjust values after stain treatment
  (for _array_element (Variables|Default|GetPlacedObjects)
    (bind _asbp_laundry_item (Utilities|Casting|CastToBP_LaundryItem _array_element))
    (Variables|/Game/_Gameplay_Albie/Blueprints/Interactable/Grabbables/BP_LaundryItem.BP_LaundryItem_C|SetIsStained _asbp_laundry_item false)
    (Variables|/Game/_Gameplay_Albie/Blueprints/Interactable/Grabbables/BP_LaundryItem.BP_LaundryItem_C|SetIsFolded _asbp_laundry_item false)
    (|CallParentFunction)))

(fn ConstructionScript
  (|CallParentFunction))

(fn CanbeProcessed
  (bind _canbeprocessed (|CallParentFunction))
  (if _canbeprocessed
    (for _array_element (Variables|Default|GetPlacedObjects)
      (bind _asbp_laundry_item (Utilities|Casting|CastToBP_LaundryItem _array_element)
        (:then
          (if (not (Variables|/Game/_Gameplay_Albie/Blueprints/Interactable/Grabbables/BP_LaundryItem.BP_LaundryItem_C|GetIsStained _asbp_laundry_item))
            ;[0.05 0.05 0.05] Invalid
            (return false)))
        (:CastFailed
          (return false))))
    ;[0.05 0.05 0.05] Valid
    (return true)
    (else
      (return false))))