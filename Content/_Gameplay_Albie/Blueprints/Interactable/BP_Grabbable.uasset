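; BP_Grabbable is an interactable physics object that a player can pick up when not already holding another object.
; On grab it turns off simulation and collision on its Box and Mesh, then hands itself to the player's Grab function.
; Drop detaches it in world space and restores physics and collision.
; Every tick it sets the Box's linear velocity to the actor's velocity clamped to a maximum speed.
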(event Custom|Drop
  (bind _box (Variables|Default|GetBox))
  ;[0.05 0.05 0.05] Drop
  (Transformation|DetachFromActor "KeepWorld" "KeepWorld" "KeepWorld")
  (Physics|SetSimulatePhysics _box true)
  (Collision|SetCollisionEnabled _box "QueryAndPhysics"))

(event Custom|Grab
  (params (Player :type BP%20Character%20Object%20Reference))
  ;[0.05 0.05 0.05] Grab
  (CallFunction|RemovePhysics)
  (Default|Grab Player self))

(event EventTick
  (params (DeltaSeconds :type Float%20%28single-precision%29))
  ;[0.05 0.05 0.05] Set Max Velocity
  (Physics|SetPhysicsLinearVelocity (Variables|Default|GetBox) (Math|Vector|ClampVectorSize (Transformation|GetVelocity) 0.0 2.5e+02) false "None"))

(event EventGrab/Drop
  (params (Player :type BP%20Character%20Object%20Reference))
  ;[0.05 0.05 0.05] Grab/Drop
  (if (CallFunction|CanbeGrabbed Player)
    (CallFunction|Grab Player)
    (Collision|SetCollisionEnabled (Variables|Default|GetMesh) "NoCollision")))

(fn ConstructionScript)

(fn CanbeGrabbed
  (params (Player :type BP%20Character%20Object%20Reference))
  (return (not (.ReturnValue (Default|GetGrabbedObject Player)))))

(fn RemovePhysics
  (bind _box (Variables|Default|GetBox))
  (Physics|SetSimulatePhysics _box false)
  (Collision|SetCollisionEnabled _box "NoCollision"))