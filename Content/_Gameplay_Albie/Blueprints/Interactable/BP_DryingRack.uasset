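; BP_DryingRack is an interactable processing station that dries wet laundry items placed on it.
; It overrides Place to accept only wet BP_LaundryItems and start processing, and disables the inherited interact inputs.
; When processing finishes, the last object is marked dry and has its mesh state updated.
; Grabbing an item resets progress, hides the progress bar and stops the progress timer.
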(event EventBeginPlay
  ;[0.05 0.05 0.05] Interact Overrides - to do nothing
)

(event EventFinishProcess
  ;[0.05 0.05 0.05] Adjust values
  (bind _output (CallFunction|GetLastObject))
  (bind _asbp_laundry_item (Utilities|Casting|CastToBP_LaundryItem _output))
  (Variables|/Game/_Gameplay_Albie/Blueprints/Interactable/Grabbables/BP_LaundryItem.BP_LaundryItem_C|SetIsWet _asbp_laundry_item false)
  (Default|UpdateMeshState _asbp_laundry_item)
  (|CallParentFunction))

(event EventGrab
  (params (Player :type BP%20Character%20Object%20Reference))
  ;[0.05 0.05 0.05] Grab Override
  (Variables|Default|SetProgress 0.0)
  (Rendering|SetVisibility (Variables|Default|GetProgressBar) false false)
  (Variables|Default|SetIsActive false)
  (Utilities|Time|ClearTimerbyFunctionName 0 "UpdateProgress")
  (|CallParentFunction Player))

(event EventInteract
  (params (player :type BP%20Character%20Object%20Reference))
  ;[0.05 0.05 0.05] Interact Overrides - to do nothing
)

(event EventHoldInteract
  (params (Player :type BP%20Character%20Object%20Reference))
  ;[0.05 0.05 0.05] Interact Overrides - to do nothing
)

(event EventTapInteract
  (params (Player :type BP%20Character%20Object%20Reference))
  ;[0.05 0.05 0.05] Interact Overrides - to do nothing
)

(event EventPlace
  (params (Player :type BP%20Character%20Object%20Reference) (ObjectToPlace :type BP%20Grabbable%20Object%20Reference))
  ;[0.05 0.05 0.05] Place Override
  (bind _asbp_laundry_item (Utilities|Casting|CastToBP_LaundryItem ObjectToPlace))
  (if (Variables|/Game/_Gameplay_Albie/Blueprints/Interactable/Grabbables/BP_LaundryItem.BP_LaundryItem_C|GetIsWet _asbp_laundry_item)
    (|CallParentFunction Player ObjectToPlace)
    (CallFunction|ProcessItems)))

(fn ConstructionScript
  (|CallParentFunction))