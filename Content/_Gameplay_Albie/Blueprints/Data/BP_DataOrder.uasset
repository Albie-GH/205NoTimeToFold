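; BP_DataOrder holds the state of a single timed order, tracking whether it is active, completed or failed on time.
; Starting it runs a looping timer that counts down the remaining time and updates the order widget's progress.
; Completion stops the timer and marks the order done, while expiry stops it, flags a time fail and notifies the GameState, leaving the active flag set.
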(event Custom|StartTimer
  ;[0.05 0.05 0.05] Set timer and update
  (Variables|Default|SetTimeRemaining (Variables|Default|GetTimeTotal))
  (Utilities|Time|SetTimerbyEvent (delegate Custom|UpdateTimer) (Variables|Default|GetTimeUpdateInterval) true))

(event Custom|UpdateTimer
  ;[0.05 0.05 0.05] Set timer and update
  (bind _output_get (Variables|Default|SetTimeRemaining (- (Variables|Default|GetTimeRemaining) (Variables|Default|GetTimeUpdateInterval))))
  (Default|UpdateProgress (Variables|Default|GetOrderWidget) _output_get (Variables|Default|GetTimeTotal))
  ;[0.05 0.05 0.05] Fail if time runs out
  (if (<= (Variables|Default|GetTimeRemaining) 0.0)
    (CallFunction|FailOrder)))

(event Custom|StartOrder
  ;[0.05 0.05 0.05] Call to start order
  (Variables|Default|SetIsActive true)
  (CallFunction|StartTimer))

(event Custom|CompleteOrder
  ;[0.05 0.05 0.05] Complete Order
  (Variables|Default|SetIsActive false)
  (Variables|Default|SetIsComplete true)
  (Utilities|Time|ClearTimerbyFunctionName 0 "UpdateTimer"))

(event Custom|FailOrder
  (Variables|Default|SetTimeFail true)
  (Utilities|Time|ClearTimerbyFunctionName 0 "UpdateTimer")
  (Default|FailOrder (Variables|Default|GetGameState) self (Variables|Default|GetOrderWidget))
  ;[1 1 1] Debug
  (Development|PrintString 0 "TIME FAIL!"))