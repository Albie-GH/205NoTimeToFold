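; BP_DataItem is an item data Blueprint that chooses which image enum represents the item from its color and delicate flag.
; SetIconEnum fills ColorMap with every pairing of four color values and the IsDelicate boolean, each mapped to one of eight image enum values.
; It then looks up the item's own Color and IsDelicate pair and stores the result in ItemImageEnum.
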(fn SetIconEnum
  (Utilities|FlowControl|Sequence
    (:then_0
      (Utilities|Map|Add (Variables|Default|GetColorMap) (Utilities|Struct|MakeFItemImageStruct "NewEnumerator0" false) "NewEnumerator0"))
    (:then_1
      (Utilities|Map|Add (Variables|Default|GetColorMap) (Utilities|Struct|MakeFItemImageStruct "NewEnumerator0" true) "NewEnumerator4"))
    (:then_2
      (Utilities|Map|Add (Variables|Default|GetColorMap) (Utilities|Struct|MakeFItemImageStruct "NewEnumerator1" false) "NewEnumerator1"))
    (:then_3
      (Utilities|Map|Add (Variables|Default|GetColorMap) (Utilities|Struct|MakeFItemImageStruct "NewEnumerator1" true) "NewEnumerator5"))
    (:then_4
      (Utilities|Map|Add (Variables|Default|GetColorMap) (Utilities|Struct|MakeFItemImageStruct "NewEnumerator2" false) "NewEnumerator3"))
    (:then_5
      (Utilities|Map|Add (Variables|Default|GetColorMap) (Utilities|Struct|MakeFItemImageStruct "NewEnumerator2" true) "NewEnumerator7"))
    (:then_6
      (Utilities|Map|Add (Variables|Default|GetColorMap) (Utilities|Struct|MakeFItemImageStruct "NewEnumerator3" false) "NewEnumerator2"))
    (:then_7
      (Utilities|Map|Add (Variables|Default|GetColorMap) (Utilities|Struct|MakeFItemImageStruct "NewEnumerator3" true) "NewEnumerator6"))
    (:then_8
      (Variables|Default|SetItemImageEnum (.Value (Utilities|Map|Find (Variables|Default|GetColorMap) (Utilities|Struct|MakeFItemImageStruct (Variables|Default|GetColor) (Variables|Default|GetIsDelicate))))))))