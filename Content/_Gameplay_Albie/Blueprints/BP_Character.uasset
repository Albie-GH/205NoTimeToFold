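; Player character Blueprint that moves via Enhanced Input, grabs and drops objects, and starts or stops interactions with world objects.
; Grab and interact inputs sphere-trace ahead on separate channels, choosing the hit best aligned with facing by 2D dot product.
; The chosen actor receives a message with the character.
; Grab attaches objects to Hands, while SetIsInteracting stores the active object so StopInteraction can end it.
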(event Custom|Grab
  (params (ObjectToGrab :type BP%20Grabbable%20Object%20Reference))
  ;[0.05 0.05 0.05] Grab
  (bind _output_get (Variables|Default|SetGrabbedObject ObjectToGrab))
  (Transformation|AttachComponentToComponent _output_get (Variables|Default|GetHands) "None" "KeepWorld" "KeepWorld" "KeepWorld" true)
  (Components|MoveComponentTo (Variables|/Script/Engine.Actor|GetRootComponent (Variables|Default|GetGrabbedObject)) "0, 0, 0" "0, 0, 0" false false 0.2 false))

(event Custom|SetIsInteracting
  (params (Interacting :type Boolean) (InteractingObject :type BPI%20Interactable%20Interface))
  ;[0.05 0.05 0.05] Set IsInteracting
  (Variables|Default|SetIsInteracting Interacting)
  (Variables|Default|SetInteracting%20Object InteractingObject))

(event Custom|StopInteraction
  (bind _interacting_object (Variables|Default|GetInteracting%20Object))
  ;[0.05 0.05 0.05] Stop Interacting
  (Utilities|IsValid (Utilities|ToObject(Interface) _interacting_object)
    (:Is%20Valid
      (Default|StopInteraction _interacting_object))))

(event Input|EnhancedActionEvents|EnhancedInputActionIA_Movement
  (params (ActionValue :type Vector%202D%20Structure) (ElapsedSeconds :type Float%20%28double-precision%29) (TriggeredSeconds :type Float%20%28double-precision%29) (InputAction :type Input%20Action%20Object%20Reference :default "/Game/_Gameplay_Albie/Inputs/IA_Movement.IA_Movement"))
  ;[0.05 0.05 0.05] Movement
  (Pawn|Input|AddMovementInput (Math|Conversions|ToVector(Vector2D) ActionValue) 1.0 false))

(event Input|EnhancedActionEvents|EnhancedInputActionIA_GrabDrop
  (params (ActionValue :type Boolean) (ElapsedSeconds :type Float%20%28double-precision%29) (TriggeredSeconds :type Float%20%28double-precision%29) (InputAction :type Input%20Action%20Object%20Reference :default "/Game/_Gameplay_Albie/Inputs/IA_GrabDrop.IA_GrabDrop"))
  (bind (_returnvalue _grabbedobject) (CallFunction|GetGrabbedObject))
  ;[0.05 0.05 0.05] Grab/Drop
  (:Started
    (bind (_returnvalue_2 _outhit) (CallFunction|FindObjecttoInteractWIth "TraceTypeQuery3"))
    (if _returnvalue_2
      (Class|BPIInteractable|Grab/Drop(Message) (.HitActor (Collision|BreakHitResult _outhit)) self)
      (elif _returnvalue
        (Default|Drop _grabbedobject)
        (Variables|Default|SetGrabbedObject 0)))))

(event Input|EnhancedActionEvents|EnhancedInputActionIA_StartInteraction
  (params (ActionValue :type Boolean) (ElapsedSeconds :type Float%20%28double-precision%29) (TriggeredSeconds :type Float%20%28double-precision%29) (InputAction :type Input%20Action%20Object%20Reference :default "/Game/_Gameplay_Albie/Inputs/IA_StartInteraction.IA_StartInteraction"))
  ;[0.05 0.05 0.05] Start Interaction
  (:Started
    (if (Variables|Default|GetIsInteracting)
      (CallFunction|StopInteraction)
      (else
        (bind (_returnvalue _outhit) (CallFunction|FindObjecttoInteractWIth "TraceTypeQuery4"))
        (if _returnvalue
          (Class|BPIInteractable|Interact(Message) (.HitActor (Collision|BreakHitResult _outhit)) self))))))

(event Input|EnhancedActionEvents|EnhancedInputActionIA_StopInteraction
  (params (ActionValue :type Boolean) (ElapsedSeconds :type Float%20%28double-precision%29) (TriggeredSeconds :type Float%20%28double-precision%29) (InputAction :type Input%20Action%20Object%20Reference :default "/Game/_Gameplay_Albie/Inputs/IA_StopInteraction.IA_StopInteraction"))
  ;[0.05 0.05 0.05] Stop Interacting
  (CallFunction|StopInteraction))

(fn ConstructionScript)

(fn GetGrabbedObject
  (bind _grabbedobject (Variables|Default|GetGrabbedObject))
  (return (Utilities|IsValid _grabbedobject) _grabbedobject))

(fn FindObjecttoInteractWIth
  (params (TraceChannel :type ETraceTypeQuery%20Enum :default "TraceTypeQuery1"))
  (bind _returnvalue (Transformation|GetActorForwardVector))
  (bind _returnvalue_2 (Transformation|GetActorLocation))
  (bind _returnvalue_3 (* _returnvalue 5e+01))
  (bind _returnvalue_4 (+ _returnvalue_3 _returnvalue_2))
  (bind (_x _y _z) (Math|Vector|BreakVector _returnvalue_4))
  ;[0.05 0.05 0.05] Create sphere traces
  (bind (_outhits _returnvalue_5) (Collision|MultiSphereTraceByChannel (Math|Vector|MakeVector _x _y (- _z 5e+01)) (Math|Vector|MakeVector _x _y (+ _z 1e+01)) 5e+01 TraceChannel false (Utilities|Array|MakeArray (Variables|Default|GetGrabbedObject)) "ForDuration" true "(R=1.000000,G=0.000000,B=0.000000,A=1.000000)" "(R=0.000000,G=1.000000,B=0.000000,A=1.000000)" 1.0))
  ;[0.05 0.05 0.05] Check which hit result is most aligned with player FOV
  (for _array_element _outhits
    ;;[0.05 0.05 0.05] Compare player forward vector with hit direction
    (if (> (Math|Vector|DotProduct (Math|Vector|Normalize (Math|Conversions|ToVector(Vector2D) (Math|Conversions|ToVector2D(Vector) (Transformation|GetActorForwardVector)))) (Math|Vector|Normalize (Math|Conversions|ToVector(Vector2D) (- (Transformation|GetActorLocation (.HitActor (Collision|BreakHitResult _array_element))) (Transformation|GetActorLocation))))) (LocalVariables|GetMostAligned))
      (LocalVariables|SetMostAligned (Math|Vector|DotProduct (Math|Vector|Normalize (Math|Conversions|ToVector(Vector2D) (Math|Conversions|ToVector2D(Vector) (Transformation|GetActorForwardVector)))) (Math|Vector|Normalize (Math|Conversions|ToVector(Vector2D) (- (Transformation|GetActorLocation (.HitActor (Collision|BreakHitResult _array_element))) (Transformation|GetActorLocation))))))
      (LocalVariables|SetMostAlignedActor _array_element)))
  ;[0.05 0.05 0.05] Return most aligned hit result actor
  (return _returnvalue_5 (LocalVariables|GetMostAlignedActor)))