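; Game mode that points the first player's view at a CameraActor on BeginPlay and applies saved audio settings.
; LoadSoundSettings loads the SaveSetings slot, or creates an unsaved default object, then sets Master, Music and SFX sound mix overrides, with zero volume when muted.
; Master reads the Music mute flag rather than one of its own.
; ReloadCurrentLevel restores game-only input and reopens the current level.
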(event Custom|ReloadCurrentLevel
  ;[0.05 0.05 0.05] Reload Level
  (Input|SetInputModeGameOnly (Game|GetPlayerController 0) false)
  (bind _returnvalue (Game|GetCurrentLevelName true))
  (Game|OpenLevel(byName) (Utilities|String|StringToName _returnvalue)))

(event EventBeginPlay
  ;[0.05 0.05 0.05] Start
  (bind _returnvalue (Actor|GetActorOfClass "/Script/Engine.CameraActor"))
  (Game|Player|SetViewTargetwithBlend (Game|GetPlayerController 0) _returnvalue 0.0 "VTBlend_Linear" 0.0 false)
  (CallFunction|LoadSoundSettings))

(event EventTick
  (params (DeltaSeconds :type Float%20%28single-precision%29)))

(fn ConstructionScript)

(fn LoadSoundSettings
  ;[0.05 0.05 0.05] Load Sound Settings
  (bind _returnvalue (SaveGame|DoesSaveGameExist (LocalVariables|GetSavefile)))
  (if _returnvalue
    (bind _returnvalue_2 (SaveGame|LoadGamefromSlot (LocalVariables|GetSavefile)))
    (bind _assave_setings (Utilities|Casting|CastToSaveSetings _returnvalue_2))
    (LocalVariables|SetSaveSetingsRef _assave_setings)
    (else
      (bind _returnvalue_3 (SaveGame|CreateSaveGameObject "/Game/Aedan_UI/Savegame/SaveSetings.SaveSetings_C"))
      (LocalVariables|SetSaveSetingsRef _returnvalue_3)))
  (Utilities|FlowControl|Sequence
    (:then_0
      (Audio|SetSoundMixClassOverride 0 "/Game/Aedan_UI/Sounds/Classes/Master.Master" (Math|Float|SelectFloat 0.0 (Variables|/Game/Aedan_UI/Savegame/SaveSetings.SaveSetings_C|GetMasterVolumeValue (LocalVariables|GetSaveSetingsRef)) (Variables|/Game/Aedan_UI/Savegame/SaveSetings.SaveSetings_C|GetMusicIsMutedBool (LocalVariables|GetSaveSetingsRef))) 1.0 0.0 true)
      (Audio|PushSoundMixModifier "/Game/Aedan_UI/Sounds/Classes/SOUND_MIX.SOUND_MIX"))
    (:then_1
      (Audio|SetSoundMixClassOverride 0 "/Game/Aedan_UI/Sounds/Classes/Music.Music" (Math|Float|SelectFloat 0.0 (Variables|/Game/Aedan_UI/Savegame/SaveSetings.SaveSetings_C|GetMusicVolumeValue (LocalVariables|GetSaveSetingsRef)) (Variables|/Game/Aedan_UI/Savegame/SaveSetings.SaveSetings_C|GetMusicIsMutedBool (LocalVariables|GetSaveSetingsRef))) 1.0 0.0 true)
      (Audio|PushSoundMixModifier "/Game/Aedan_UI/Sounds/Classes/SOUND_MIX.SOUND_MIX"))
    (:then_2
      (Audio|SetSoundMixClassOverride 0 "/Game/Aedan_UI/Sounds/Classes/SFX.SFX" (Math|Float|SelectFloat 0.0 (Variables|/Game/Aedan_UI/Savegame/SaveSetings.SaveSetings_C|GetSfxVolumeValue (LocalVariables|GetSaveSetingsRef)) (Variables|/Game/Aedan_UI/Savegame/SaveSetings.SaveSetings_C|GetSfxIsMutedBool (LocalVariables|GetSaveSetingsRef))) 1.0 0.0 true)
      (Audio|PushSoundMixModifier "/Game/Aedan_UI/Sounds/Classes/SOUND_MIX.SOUND_MIX")))
  (return))