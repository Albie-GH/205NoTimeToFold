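; Game state for a laundry level that runs the level timer, generates random customer orders and tracks score.
; At BeginPlay it builds the laundry mesh map, pre-generates all orders from random item data objects and creates the level and order HUDs.
; A looping timer spawns a laundry bag on the tagged counter; its first pickup activates the order and its HUD widget.
; Completed orders are scored from item rewards, quality penalties and a time-remaining multiplier.
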(event Custom|SpawnOrder
  (bind _allorders (Variables|Orders|GetAllOrders))
  (bind _orderspawnindex (Variables|Orders|GetOrderSpawnIndex))
  (bind _output (Utilities|Array|Get(acopy) _allorders _orderspawnindex))
  (bind _orderitems (Variables|/Game/_Gameplay_Albie/Blueprints/Data/BP_DataOrder.BP_DataOrder_C|GetOrderItems _output))
  ;[0.05 0.05 0.05] Spawn customer order on counter
  (bind _outactors (Actor|GetAllActorsOfClasswithTag "/Game/_Gameplay_Albie/Blueprints/Interactable/BP_Counter.BP_Counter_C" "OrderSpawner"))
  (if (Utilities|Array|IsEmpty (Variables|/Game/_Gameplay_Albie/Blueprints/Interactable/BP_Interactable.BP_Interactable_C|GetPlacedObjects (Utilities|Array|Get(acopy) _outactors)))
    (Variables|/Game/_Gameplay_Albie/Blueprints/Interactable/BP_Counter.BP_Counter_C|SetSpawnActorClass (Utilities|Array|Get(acopy) _outactors) "/Game/_Gameplay_Albie/Blueprints/Interactable/Grabbables/BP_LaundryBag.BP_LaundryBag_C")
    (bind _returnvalue (Game|SpawnActorfromClass "/Game/_Gameplay_Albie/Blueprints/Interactable/Grabbables/BP_LaundryBag.BP_LaundryBag_C" (Transformation|GetActorTransform (Utilities|Array|Get(acopy) _outactors)) "Undefined" "MultiplyWithRoot" 0 0 0))
    (bind _output_get (Variables|Default|SetNextOrderRef _returnvalue))
    (EventDispatchers|BindEventtoOnFirstPickUp _output_get (delegate Custom|AddNextOrder))
    (Default|InitItems _returnvalue _orderitems (Variables|Default|GetLaundryMeshMap))
    (Variables|/Game/_Gameplay_Albie/Blueprints/Interactable/BP_Counter.BP_Counter_C|SetLaundryBagTest (Utilities|Array|Get(acopy) _outactors) _returnvalue)
    (Default|SpawnonCounter (Utilities|Array|Get(acopy) _outactors) _returnvalue)
    ;[1 1 1] Debug
    (for _array_element _orderitems
      (Development|PrintText (Utilities|Text|FormatText "Color: {c} 
Delicate: {d} 
Airdry: {a} 
Stain: {s}" (Utilities|String|EnumtoString (Variables|/Game/_Gameplay_Albie/Blueprints/Data/BP_DataItem.BP_DataItem_C|GetColor _array_element)) (Variables|/Game/_Gameplay_Albie/Blueprints/Data/BP_DataItem.BP_DataItem_C|GetIsDelicate _array_element) (Variables|/Game/_Gameplay_Albie/Blueprints/Data/BP_DataItem.BP_DataItem_C|GetAirDryOnly _array_element) (Variables|/Game/_Gameplay_Albie/Blueprints/Data/BP_DataItem.BP_DataItem_C|GetIsStained _array_element))))))

(event Custom|AddOrderToHUD
  (bind _allorders (Variables|Orders|GetAllOrders))
  (bind _orderspawnindex (Variables|Orders|GetOrderSpawnIndex))
  (bind _output (Utilities|Array|Get(acopy) _allorders _orderspawnindex))
  ;[0.05 0.05 0.05] Add order widget  to HUD and start timer
  (bind _returnvalue (UserInterface|CreateWidget "/Game/UI_OrderSystem/WBP_OrderWidget.WBP_OrderWidget_C"))
  (Default|InitItems _returnvalue (Variables|/Game/_Gameplay_Albie/Blueprints/Data/BP_DataOrder.BP_DataOrder_C|GetOrderItems _output))
  (Default|CreateOrderItems _returnvalue)
  (Default|AddOrder (Variables|HUD|GetOrderHUDRef) _returnvalue)
  (Variables|/Game/_Gameplay_Albie/Blueprints/Data/BP_DataOrder.BP_DataOrder_C|SetOrderWidget _output _returnvalue)
  (Default|StartOrder _output)
  (Default|DecreaseOrderNumber (Variables|HUD|GetMainHUDRef)))

(event Custom|StartTimer
  ;[0.05 0.05 0.05] Level Timer
  (Variables|Time|SetLevelTimeRemaining (Variables|Time|GetLevelTime))
  (Utilities|Time|SetTimerbyEvent (delegate Custom|UpdateTimer) (Variables|Time|GetTimeUpdateInterval) true))

(event Custom|UpdateTimer
  ;[0.05 0.05 0.05] Level Timer
  (Variables|Time|SetLevelTimeRemaining (- (Variables|Time|GetLevelTimeRemaining) (Variables|Time|GetTimeUpdateInterval)))
  (Default|SetRemainingTime (Variables|HUD|GetMainHUDRef) (/ (Variables|Time|GetLevelTimeRemaining) (Variables|Time|GetLevelTime))))

(event Custom|SpawnNextOrder
  ;[0.05 0.05 0.05] Adding Orders
  (if (< (Variables|Orders|GetOrderSpawnIndex) (Variables|Orders|GetTotalOrdersForLevel))
    (if (< (Utilities|Array|Length (Variables|Orders|GetActiveOrders)) (Variables|Orders|GetMaxActiveOrders))
      (CallFunction|SpawnOrder))
    (else
      (Utilities|Time|ClearTimerbyFunctionName 0 "SpawnNextOrder"))))

(event Custom|StartOrderTimer
  ;[0.05 0.05 0.05] Adding Orders
  (Utilities|Time|SetTimerbyEvent (delegate Custom|SpawnNextOrder) (Variables|Time|GetOrderSpawnInterval) true (Variables|Time|GetOrderStartDelay)))

(event Custom|AddNextOrder
  ;[0.05 0.05 0.05] Spawn customer order on counter
  (CallFunction|AddtoActiveOrders (Utilities|Array|Get(acopy) (Variables|Orders|GetAllOrders) (Variables|Orders|GetOrderSpawnIndex)))
  (Default|AddBasket (Variables|Default|GetBasketStand))
  (CallFunction|AddOrdertoHUD)
  (Math|Integer|IncrementInt (Variables|Orders|GetOrderSpawnIndex)))

(event EventBeginPlay
  (CallFunction|PopulateLaundryMeshMap)
  (CallFunction|GenerateOrdersArray)
  ;[0.05 0.05 0.05] Main HUD
  (bind _returnvalue (UserInterface|CreateWidget "/Game/_Gameplay_Albie/Blueprints/UI/WBP_LevelHUD.WBP_LevelHUD_C"))
  (bind _output_get (Variables|HUD|SetMainHUDRef _returnvalue))
  (Default|SetOrderNumber _output_get (Variables|Orders|GetTotalOrdersForLevel))
  (UserInterface|Viewport|AddtoViewport _returnvalue 0)
  ;[0.05 0.05 0.05] Order HUD - Add to main HUD?
  (bind _returnvalue_2 (UserInterface|CreateWidget "/Game/UI_OrderSystem/WBP_OrderHUD.WBP_OrderHUD_C"))
  (Variables|HUD|SetOrderHUDRef _returnvalue_2)
  (UserInterface|Viewport|AddtoViewport _returnvalue_2 0)
  (CallFunction|StartTimer)
  (CallFunction|StartOrderTimer))

(fn ConstructionScript
  (bind _returnvalue (Utilities|LoadClassAssetBlocking "/Game/_Gameplay_Albie/Blueprints/Data/BP_DataItem.BP_DataItem_C"))
  (Variables|Default|SetDataItemClass _returnvalue)
  (CallFunction|PopulateLaundryMeshMap))

(fn GenerateOrdersArray
  ;[0.05 0.05 0.05] Loop to generate orders
  (for _index (range 0 (- (Variables|Orders|GetTotalOrdersForLevel) 1))
    ;[0.05 0.05 0.05] Add generated orders to Orders array
    (bind _returnvalue (Game|ConstructObjectfromClass "/Game/_Gameplay_Albie/Blueprints/Data/BP_DataOrder.BP_DataOrder_C" self))
    (Utilities|Array|Add (Variables|Orders|GetAllOrders) _returnvalue)
    ;[0.05 0.05 0.05] Loop to generate and add order items
    (for _index_2 (range 1 (Math|Random|RandomIntegerinRange 1 (Variables|Orders|GetMaxItemsPerOrder)))
      (bind _laundryitemdata (CallFunction|GenerateOrderItem))
      (Utilities|Array|Add (Variables|/Game/_Gameplay_Albie/Blueprints/Data/BP_DataOrder.BP_DataOrder_C|GetOrderItems (Utilities|Array|Get(acopy) (Variables|Orders|GetAllOrders) _index)) _laundryitemdata))))

(fn GenerateOrderItem
  (bind _returnvalue (Game|ConstructObjectfromClass (Variables|Default|GetDataItemClass)))
  (bind _asbp_data_item (Utilities|Casting|CastToBP_DataItem _returnvalue))
  (Variables|/Game/_Gameplay_Albie/Blueprints/Data/BP_DataItem.BP_DataItem_C|SetColor _asbp_data_item (Utilities|Select :Index (Math|Random|RandomIntegerinRange 0 3) :Option%200 "NewEnumerator0" :Option%201 "NewEnumerator1" :Option%202 "NewEnumerator2" :Option%203 "NewEnumerator3"))
  (Variables|/Game/_Gameplay_Albie/Blueprints/Data/BP_DataItem.BP_DataItem_C|SetIsDelicate _asbp_data_item (Math|Random|RandomBool))
  (Variables|/Game/_Gameplay_Albie/Blueprints/Data/BP_DataItem.BP_DataItem_C|SetAirDryOnly _asbp_data_item (Math|Random|RandomBool))
  (Variables|/Game/_Gameplay_Albie/Blueprints/Data/BP_DataItem.BP_DataItem_C|SetIsStained _asbp_data_item (Math|Random|RandomBool))
  (Default|SetIconEnum _asbp_data_item)
  (return _asbp_data_item))

(fn PopulateLaundryMeshMap
  (Utilities|FlowControl|Sequence
    (:then_0
      ;[0.05 0.05 0.05] White
      (Utilities|Map|Add (Variables|Default|GetLaundryMeshMap) (Utilities|Struct|MakeFLaundryMeshStruct "NewEnumerator0" "NewEnumerator1" false false) "/Game/_John_ArtAssets/Mesh/Interactables/Clothes/MDL_CLWH_dirty.MDL_CLWH_dirty")
      (Utilities|Map|Add (Variables|Default|GetLaundryMeshMap) (Utilities|Struct|MakeFLaundryMeshStruct "NewEnumerator0" "NewEnumerator1" true false) "/Game/_John_ArtAssets/Mesh/Interactables/Clothes/MDL_CLWH_dirty.MDL_CLWH_dirty")
      (Utilities|Map|Add (Variables|Default|GetLaundryMeshMap) (Utilities|Struct|MakeFLaundryMeshStruct "NewEnumerator0" "NewEnumerator3" false true) "/Game/_John_ArtAssets/Mesh/Interactables/Clothes/MDL_CLWH_folded.MDL_CLWH_folded")
      (Utilities|Map|Add (Variables|Default|GetLaundryMeshMap) (Utilities|Struct|MakeFLaundryMeshStruct "NewEnumerator0" "NewEnumerator3" false false) "/Game/_John_ArtAssets/Mesh/Interactables/Clothes/MDL_CLWH_unfolded.MDL_CLWH_unfolded")
      (Utilities|Map|Add (Variables|Default|GetLaundryMeshMap) (Utilities|Struct|MakeFLaundryMeshStruct "NewEnumerator0" "NewEnumerator3" true false) "/Game/_John_ArtAssets/Mesh/Interactables/Clothes/MDL_CLWH_wet.MDL_CLWH_wet"))
    (:then_1
      ;[0.05 0.05 0.05] Red
      (Utilities|Map|Add (Variables|Default|GetLaundryMeshMap) (Utilities|Struct|MakeFLaundryMeshStruct "NewEnumerator1" "NewEnumerator1" false false) "/Game/_John_ArtAssets/Mesh/Interactables/Clothes/MDL_CLRE_dirty.MDL_CLRE_dirty")
      (Utilities|Map|Add (Variables|Default|GetLaundryMeshMap) (Utilities|Struct|MakeFLaundryMeshStruct "NewEnumerator1" "NewEnumerator1" true false) "/Game/_John_ArtAssets/Mesh/Interactables/Clothes/MDL_CLRE_dirty.MDL_CLRE_dirty")
      (Utilities|Map|Add (Variables|Default|GetLaundryMeshMap) (Utilities|Struct|MakeFLaundryMeshStruct "NewEnumerator1" "NewEnumerator3" false true) "/Game/_John_ArtAssets/Mesh/Interactables/Clothes/MDL_CLRE_folded.MDL_CLRE_folded")
      (Utilities|Map|Add (Variables|Default|GetLaundryMeshMap) (Utilities|Struct|MakeFLaundryMeshStruct "NewEnumerator1" "NewEnumerator3" false false) "/Game/_John_ArtAssets/Mesh/Interactables/Clothes/MDL_CLRE_unfolded.MDL_CLRE_unfolded")
      (Utilities|Map|Add (Variables|Default|GetLaundryMeshMap) (Utilities|Struct|MakeFLaundryMeshStruct "NewEnumerator1" "NewEnumerator3" true false) "/Game/_John_ArtAssets/Mesh/Interactables/Clothes/MDL_CLRE_wet.MDL_CLRE_wet"))
    (:then_2
      ;[0.05 0.05 0.05] Green
      (Utilities|Map|Add (Variables|Default|GetLaundryMeshMap) (Utilities|Struct|MakeFLaundryMeshStruct "NewEnumerator2" "NewEnumerator1" false false) "/Game/_John_ArtAssets/Mesh/Interactables/Clothes/MDL_CLGR_dirty.MDL_CLGR_dirty")
      (Utilities|Map|Add (Variables|Default|GetLaundryMeshMap) (Utilities|Struct|MakeFLaundryMeshStruct "NewEnumerator2" "NewEnumerator1" true false) "/Game/_John_ArtAssets/Mesh/Interactables/Clothes/MDL_CLGR_dirty.MDL_CLGR_dirty")
      (Utilities|Map|Add (Variables|Default|GetLaundryMeshMap) (Utilities|Struct|MakeFLaundryMeshStruct "NewEnumerator2" "NewEnumerator3" false true) "/Game/_John_ArtAssets/Mesh/Interactables/Clothes/MDL_CLGR_folded.MDL_CLGR_folded")
      (Utilities|Map|Add (Variables|Default|GetLaundryMeshMap) (Utilities|Struct|MakeFLaundryMeshStruct "NewEnumerator2" "NewEnumerator3" false false) "/Game/_John_ArtAssets/Mesh/Interactables/Clothes/MDL_CLGR_unfolded.MDL_CLGR_unfolded")
      (Utilities|Map|Add (Variables|Default|GetLaundryMeshMap) (Utilities|Struct|MakeFLaundryMeshStruct "NewEnumerator2" "NewEnumerator3" true false) "/Game/_John_ArtAssets/Mesh/Interactables/Clothes/MDL_CLGR_wet.MDL_CLGR_wet"))
    (:then_3
      ;[0.05 0.05 0.05] Blue
      (Utilities|Map|Add (Variables|Default|GetLaundryMeshMap) (Utilities|Struct|MakeFLaundryMeshStruct "NewEnumerator3" "NewEnumerator1" false false) "/Game/_John_ArtAssets/Mesh/Interactables/Clothes/MDL_CLBL_dirty.MDL_CLBL_dirty")
      (Utilities|Map|Add (Variables|Default|GetLaundryMeshMap) (Utilities|Struct|MakeFLaundryMeshStruct "NewEnumerator3" "NewEnumerator1" true false) "/Game/_John_ArtAssets/Mesh/Interactables/Clothes/MDL_CLBL_dirty.MDL_CLBL_dirty")
      (Utilities|Map|Add (Variables|Default|GetLaundryMeshMap) (Utilities|Struct|MakeFLaundryMeshStruct "NewEnumerator3" "NewEnumerator3" false true) "/Game/_John_ArtAssets/Mesh/Interactables/Clothes/MDL_CLBL_folded.MDL_CLBL_folded")
      (Utilities|Map|Add (Variables|Default|GetLaundryMeshMap) (Utilities|Struct|MakeFLaundryMeshStruct "NewEnumerator3" "NewEnumerator3" false false) "/Game/_John_ArtAssets/Mesh/Interactables/Clothes/MDL_CLBL_unfolded.MDL_CLBL_unfolded")
      (Utilities|Map|Add (Variables|Default|GetLaundryMeshMap) (Utilities|Struct|MakeFLaundryMeshStruct "NewEnumerator3" "NewEnumerator3" true false) "/Game/_John_ArtAssets/Mesh/Interactables/Clothes/MDL_CLBL_wet.MDL_CLBL_wet"))
    (:then_4
      (return (Variables|Default|GetLaundryMeshMap)))))

(fn SetBasketStandReference
  (params (BasketStand :type BP%20Basket%20Stand%20Object%20Reference))
  (Variables|Default|SetBasketStand BasketStand))

(fn CompleteOrder
  (params (CompletedOrder :type BP%20Data%20Order%20Object%20Reference%20%28by%20ref%29) (OrderQualityArray :type Array%20of%20BP%20Data%20Item%20Object%20References))
  (bind _allorders (Variables|Orders|GetAllOrders))
  (bind _returnvalue (Utilities|Array|FindItem _allorders CompletedOrder))
  (bind _output (Utilities|Array|Get(acopy) _allorders _returnvalue))
  (Default|CompleteOrder _output)
  (Class|PanelWidget|RemoveChild (Variables|/Game/UI_OrderSystem/WBP_OrderHUD.WBP_OrderHUD_C|GetOrderContainer (Variables|HUD|GetOrderHUDRef)) (Variables|/Game/_Gameplay_Albie/Blueprints/Data/BP_DataOrder.BP_DataOrder_C|GetOrderWidget _output))
  (Utilities|Array|Add (Variables|Orders|GetCompletedOrders) _output)
  (Utilities|Array|RemoveItem (Variables|Orders|GetActiveOrders) _output)
  (CallFunction|AdjustScore OrderQualityArray _output))

(fn AddtoActiveOrders
  (params (NewOrder :type BP%20Data%20Order%20Object%20Reference%20%28by%20ref%29))
  (Utilities|Array|Add (Variables|Orders|GetActiveOrders) NewOrder))

(fn FailOrder
  (params (FailedOrder :type BP%20Data%20Order%20Object%20Reference%20%28by%20ref%29) (OrderWidget :type WBP%20Order%20Widget%20Object%20Reference))
  (bind _allorders (Variables|Orders|GetAllOrders))
  (bind _returnvalue (Utilities|Array|FindItem _allorders FailedOrder))
  (bind _output (Utilities|Array|Get(acopy) _allorders _returnvalue))
  (Class|PanelWidget|RemoveChild (Variables|/Game/UI_OrderSystem/WBP_OrderHUD.WBP_OrderHUD_C|GetOrderContainer (Variables|HUD|GetOrderHUDRef)) OrderWidget)
  (Utilities|Array|Add (Variables|Orders|GetFailedOrders) _output)
  (Utilities|Array|RemoveItem (Variables|Orders|GetActiveOrders) _output))

(fn AdjustScore
  (params (OrderQualityArray :type Array%20of%20BP%20Data%20Item%20Object%20References) (OrderData :type BP%20Data%20Order%20Object%20Reference))
  (bind _timebonus (CallFunction|CalculateTimeBonus OrderData))
  (LocalVariables|SetOrderTimeBonusMultiplier _timebonus)
  (for _array_element OrderQualityArray
    ;[0.05 0.05 0.05] Unfolded Penalty
    (if (not (Variables|/Game/_Gameplay_Albie/Blueprints/Data/BP_DataItem.BP_DataItem_C|GetIsFolded _array_element))
      (LocalVariables|SetOrderPenalties (+ (LocalVariables|GetOrderPenalties) (Variables|Score-Rewards|GetUnfoldedPenalty))))
    ;[0.05 0.05 0.05] Score for item
    (LocalVariables|SetOrderBaseScore (+ (LocalVariables|GetOrderBaseScore) (Variables|Score-Rewards|GetItemCompletedReward)))
    ;[0.05 0.05 0.05] Stained Penalty
    (if (Variables|/Game/_Gameplay_Albie/Blueprints/Data/BP_DataItem.BP_DataItem_C|GetIsStained _array_element)
      (LocalVariables|SetOrderPenalties (+ (LocalVariables|GetOrderPenalties) (Variables|Score-Rewards|GetStainedPenalty))))
    ;[0.05 0.05 0.05] Damage Penalties
    (for _array_element_2 (Variables|/Game/_Gameplay_Albie/Blueprints/Data/BP_DataItem.BP_DataItem_C|GetDamage _array_element)
      (LocalVariables|SetOrderPenalties (+ (LocalVariables|GetOrderPenalties) (.Value (Utilities|Map|Find (Variables|Score-Rewards|GetDamagePenalties) _array_element_2))))))
  (Development|PrintText (Utilities|Text|FormatText "Items in order: {i}" (Utilities|Array|Length OrderQualityArray)))
  ;[0.05 0.05 0.05] Calculate Total Order Score
  (bind _output_get (LocalVariables|SetTotalOrderScore (Math|Float|Floor (* (Math|Float|Truncate (- (LocalVariables|GetOrderBaseScore) (LocalVariables|GetOrderPenalties))) (LocalVariables|GetOrderTimeBonusMultiplier)))))
  ;[0.05 0.05 0.05] Calculate Order Time Bonus
  (LocalVariables|SetOrderTimeBonus (- _output_get (Math|Float|Truncate (- (LocalVariables|GetOrderBaseScore) (LocalVariables|GetOrderPenalties)))))
  ;[0.05 0.05 0.05] Total Penalties
  (Variables|Score|SetTotalPenalties (+ (Variables|Score|GetTotalPenalties) (LocalVariables|GetOrderPenalties)))
  ;[0.05 0.05 0.05] Total Time Bonus
  (Variables|Score|SetTotalTimeBonus (+ (Variables|Score|GetTotalTimeBonus) (LocalVariables|GetOrderTimeBonus)))
  ;[0.05 0.05 0.05] Total Base Score
  (Variables|Score|SetTotalBaseScore (+ (Variables|Score|GetTotalBaseScore) (LocalVariables|GetOrderBaseScore)))
  ;[0.05 0.05 0.05] Total Score
  (Variables|Score|SetTotalScore (+ (Variables|Score|GetTotalScore) (LocalVariables|GetTotalOrderScore)))
  ;[1 1 1] Debug
  (Development|PrintText (Utilities|Text|FormatText "Order Base Score: {obs} 
Order Penalties: {op} 
Order Time Bonus: {otb} 
Order Total Score: {ots} 
Total Base Score: {tbs} 
Total Pentalties: {tp} 
Total Time Bonus: {ttb} 
Total Score: {ts}" (LocalVariables|GetOrderBaseScore) (LocalVariables|GetOrderPenalties) (LocalVariables|GetOrderTimeBonus) (LocalVariables|GetTotalOrderScore) (Variables|Score|GetTotalBaseScore) (Variables|Score|GetTotalPenalties) (Variables|Score|GetTotalTimeBonus) (Variables|Score|GetTotalScore)) true true "(R=0.000000,G=0.660000,B=1.000000,A=1.000000)" 15.0))

(fn CalculateTimeBonus
  (params (OrderData :type BP%20Data%20Order%20Object%20Reference))
  (bind _output_get (LocalVariables|SetTimeRemainingPercent (/ (Variables|/Game/_Gameplay_Albie/Blueprints/Data/BP_DataOrder.BP_DataOrder_C|GetTimeRemaining OrderData) (Variables|/Game/_Gameplay_Albie/Blueprints/Data/BP_DataOrder.BP_DataOrder_C|GetTimeTotal OrderData))))
  ;[0.05 0.05 0.05] Big Bonus
  (if (>= _output_get 0.66)
    (return (Variables|Score-Rewards|GetLargeTimeBonusMultiplier))
    (else
      ;[0.05 0.05 0.05] Little Bonus
      (if (>= (LocalVariables|GetTimeRemainingPercent) 0.33)
        (return (Variables|Score-Rewards|GetSmallTimeBonusMultiplier))
        (else
          ;[0.05 0.05 0.05] No Bonus
          (return 1.0))))))